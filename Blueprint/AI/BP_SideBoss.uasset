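; Side boss AI character that wanders, drops timed grenades, chases the player on sight or perception stimulus, and damages them on overlap.
; Tick runs a camera dot-product and distance check; when watched up close, it flees to random navmesh points or smoke-vanishes and teleports.
; Taking damage also triggers a delayed vanish, and zero health plays a death animation and disables AI.
; Knife-throw, stun and speed events are exposed, but not called here.
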(event OnTargetPerceptionUpdated(AIPerception)
  (params (Actor :type Actor%20Object%20Reference) (Stimulus :type AI%20Stimulus%20Structure))
  (if (not (Variables|Default|GetIsInPlayerView))
    (if (Variables|Default|GetisActive)
      (if (not (Variables|Default|GetDeadBool))
        (Development|PrintString "AI Heard Sound")
        (CallFunction|SeePlayer)))))

(event OnSeePawn(PawnSensing)
  (params (Pawn :type Pawn%20Object%20Reference))
  (if (Variables|Default|GetisActive)
    (CallFunction|ChasePlayer Pawn)))

(event OnComponentBeginOverlap(HitBox)
  (params (OverlappedComponent :type Primitive%20Component%20Object%20Reference) (OtherActor :type Actor%20Object%20Reference) (OtherComp :type Primitive%20Component%20Object%20Reference) (OtherBodyIndex :type Integer) (bFromSweep :type Boolean) (SweepResult :type Hit%20Result%20Structure%20%28by%20ref%29))
  ;[1 1 1] Damage / Deal Damage
  (if (not (Variables|Default|GetDeadBool))
    (bind _asbp_player_movement (Utilities|Casting|CastToBP_PlayerMovement OtherActor))
    (if (Variables|/Script/ExtractShooter.PlayerMovement|GetDead _asbp_player_movement)
      (Variables|Default|SetDealDamage false)
      (elif (Collision|IsOverlappingActor (Variables|/Script/Engine.Character|GetMesh _asbp_player_movement) self :!class /Script/Engine.PrimitiveComponent)
        (bind _output_get (Variables|Default|SetPlayer _asbp_player_movement))
        (Variables|Default|SetDealDamage true)
        (AI|AIMoveTo self (Transformation|GetActorLocation _output_get) _asbp_player_movement 0.0 false)))))

(event OnComponentEndOverlap(HitBox)
  (params (OverlappedComponent :type Primitive%20Component%20Object%20Reference) (OtherActor :type Actor%20Object%20Reference) (OtherComp :type Primitive%20Component%20Object%20Reference) (OtherBodyIndex :type Integer))
  ;[1 1 1] Damage / Deal Damage
  (Utilities|Casting|CastToBP_PlayerMovement OtherActor)
  (Variables|Default|SetDealDamage false))

(event Custom|Dead
  ;[1 1 1] Damage / Deal Damage
  (Development|PrintString "Dead")
  (Variables|Default|SetDeadBool true)
  (Components|Animation|PlayAnimation (Variables|Character|GetMesh) "/Game/Assets/Models/Player/Dead/Falling_Forward_Death_Anim_mixamo_com.Falling_Forward_Death_Anim_mixamo_com" false)
  (CallFunction|ToggleAIFunctionality false))

(event Custom|DealDamageFunc
  (params (Player :type BP%20Player%20Movement%20Object%20Reference))
  ;[1 1 1] Damage / Deal Damage
  (if (Variables|/Script/ExtractShooter.PlayerMovement|GetDead Player)
    (Variables|Default|SetDealDamage false)
    (else
      (Variables|Default|SetCanSeePlayer true)
      (Development|PrintString "Enemy AI Hit Player")
      (Class|PlayerMovement|DealDamagetoPlayer Player (Variables|Default|GetDamage)))))

(event Custom|CheckIfInPlayerFOV
  (bind _asbp_player_movement (Utilities|Casting|CastToBP_PlayerMovement (Game|GetPlayerCharacter 0)))
  (Variables|Default|SetIsPlayerClose? (== (> (Variables|Default|GetPlayerCloseDistanceThreshold) (Math|Vector|VectorLength (- (Transformation|GetActorLocation self) (Transformation|GetActorLocation (Variables|Default|GetPlayer))))) true))
  (if (> (Math|Vector|VectorLength (- (Transformation|GetActorLocation) (Transformation|GetActorLocation _asbp_player_movement))) (Variables|Default|GetMaxViewDistance))
    (Variables|Default|SetIsInPlayerView false)
    (Variables|Default|SetRunningAway false)
    (elif (and (>= (Math|Vector|DotProduct (- (Transformation|GetActorLocation) (Transformation|GetActorLocation _asbp_player_movement)) (Math|Vector|GetForwardVector (Variables|/Game/Blueprints/Player/BP_PlayerMovement.BP_PlayerMovement_C|GetMainCamera _asbp_player_movement))) 0.5) (Variables|Default|GetIsPlayerClose?))
      (Variables|Default|SetIsInPlayerView true)
      (if (and (Variables|Default|GetIsPlayerClose?) (Variables|Default|GetIsInPlayerView))
        (Utilities|FlowControl|Delay (Variables|Default|GetVanishTimer))
        (CallFunction|Vanish))
      (if (<= (Math|Vector|VectorLength (Variables|/Script/Engine.MovementComponent|GetVelocity (Variables|Character|GetCharacterMovement))) 0.1)
        (CallFunction|RunAway))
      (else
        (Variables|Default|SetIsInPlayerView false)
        (Variables|Default|SetRunningAway false)))))

(event Custom|Chase%20Player
  (params (Pawn :type Pawn%20Object%20Reference))
  (if (not (Variables|Default|GetIsInPlayerView))
    (if (Variables|Default|GetisActive)
      (if (not (Variables|Default|GetDeadBool))
        (Utilities|Casting|CastToBP_PlayerMovement Pawn)
        (Utilities|FlowControl|Sequence
          (:then_0
            (if (Variables|Default|GetisActive)
              (CallFunction|SeePlayer)))
          (:then_1
            (if (Variables|Default|GetisActive)
              ;[1 1 1] Doesnt See Player
              (Utilities|FlowControl|RetriggerableDelay (Variables|Default|GetMemory))
              (Variables|Default|SetCanSeePlayer false))))))))

(event Custom|See%20Player
  ;[1 1 1] Chase Player As Soon As AI Sees Player
  (if (not (Variables|Default|GetIsInPlayerView))
    (Variables|Default|SetCanSeePlayer true)
    (bind _asbp_player_movement (Utilities|Casting|CastToBP_PlayerMovement (Game|GetPlayerCharacter 0)))
    (AI|AIMoveTo self (Transformation|GetActorLocation _asbp_player_movement) 0 5.0 false)))

(event Custom|TookDamage
  (Utilities|FlowControl|Delay (Variables|Default|GetTakeDamageVanishTimer))
  (CallFunction|Vanish))

(event Custom|RunAway
  (bind _returnvalue (Transformation|GetActorLocation))
  (bind _self self)
  (bind _randomlocation (AI|Navigation|GetRandomReachablePointinRadius _returnvalue 4e+03 0 0))
  (if (== (Variables|Default|GetPlayer) 0) :!label _label
    (bind _asbp_player_movement (Utilities|Casting|CastToBP_PlayerMovement (Game|GetPlayerCharacter 0)))
    (Variables|Default|SetPlayer _asbp_player_movement)
    (Utilities|FlowControl|Delay 0.2)
    (goto _label)
    (else
      (if (Variables|Default|GetRunningAway) :!label _label_2
        (if (> (Math|Vector|VectorLength (- (Transformation|GetActorLocation _self) _randomlocation)) 3e+03)
          (AI|AIMoveTo _self _randomlocation 0 5.0 true
            (:then
              (if (Variables|Default|GetIsInPlayerView)
                (if (<= (Math|Vector|VectorLength (Variables|/Script/Engine.MovementComponent|GetVelocity (Variables|Character|GetCharacterMovement))) 0.1)
                  (goto _label_2)
                  (else
                    (Utilities|FlowControl|Delay 5.0)
                    (goto _label_2)))
                (else
                  (Variables|Default|SetRunningAway false))))
            (:OnSuccess
              (Variables|Default|SetRunningAway false :!label _label_3))
            (:OnFail
              (goto _label_3)))
          (else
            (Variables|Default|SetRunningAway false)
            (goto _label_2)))
        (else
          (Variables|Default|SetRunningAway true))))))

(event Custom|Vanish
  (bind _player (Variables|Default|GetPlayer))
  (bind _charactermovement (Variables|Character|GetCharacterMovement))
  (bind _returnvalue (Transformation|GetActorLocation _player))
  (bind _randomlocation (AI|Navigation|GetRandomReachablePointinRadius _returnvalue 9e+03 0 0))
  (Variables|Default|SetVanishing true)
  (Variables|/Script/Engine.CharacterMovementComponent|SetMaxWalkSpeed _charactermovement 0.0)
  (Components|Movement|StopMovementImmediately _charactermovement)
  (CallFunction|VanishVFX)
  (if (> (Math|Vector|VectorLength (- (Transformation|GetActorLocation self) _randomlocation)) 5e+03) :!label _label
    (Transformation|SetActorLocation _randomlocation false false)
    (Variables|/Script/Engine.CharacterMovementComponent|SetMaxWalkSpeed (Variables|Character|GetCharacterMovement) 6e+02)
    (Variables|Default|SetVanishing false)
    (else
      (Utilities|FlowControl|Delay 0.2)
      (goto _label))))

(event Custom|VanishVFX
  (bind _mesh (Variables|Character|GetMesh))
  (bind _returnvalue (Transformation|GetWorldLocation _mesh))
  (Niagara|SpawnSystematLocation "/Game/Assets/Niagara/SmokeVanish/NS_SmokeVanish.NS_SmokeVanish" (Math|Vector|MakeVector (.x _returnvalue) (.y _returnvalue) (+ (.z _returnvalue) 9e+01)) "0, 0, 0" "2.000000,2.000000,2.000000"))

(event Custom|ThrowKnives
  (bind _charactermovement (Variables|Character|GetCharacterMovement))
  ;[1 1 1] Throw Stuff
  (if (== (Variables|Default|GetPlayer) 0) :!label _label
    (bind _asbp_player_movement (Utilities|Casting|CastToBP_PlayerMovement (Game|GetPlayerCharacter 0)))
    (Variables|Default|SetPlayer _asbp_player_movement)
    (Utilities|FlowControl|Delay 0.2)
    (goto _label)
    (else
      (Components|Movement|StopMovementImmediately _charactermovement)
      (Variables|/Script/Engine.CharacterMovementComponent|SetMaxWalkSpeed _charactermovement 0.0)
      (Variables|Default|SetThrowing true)
      (Utilities|FlowControl|Delay (Variables|Default|GetPreppingToThrow))
      (Utilities|FlowControl|Delay (Variables|Default|GetThrowTime))
      (bind _returnvalue (Game|SpawnActorfromClass "/Game/Blueprints/UtilityItems/BP_MainBossThrowable.BP_MainBossThrowable_C" (Math|Transform|MakeTransform (Transformation|GetWorldLocation (Variables|Default|GetThrowFromPos)) "0, 0, 0" "1.000000,1.000000,1.000000") "Undefined" 0 0))
      (Physics|AddForce (Variables|/Game/Blueprints/UtilityItems/BP_MainBossThrowable.BP_MainBossThrowable_C|GetCube _returnvalue) (* (Math|Vector|GetForwardVector (Variables|Collision|GetCapsuleComponent)) (Variables|Default|GetThrowForce)) "None" false)
      (Development|PrintString "THROWN")
      (Variables|Default|SetThrowing false)
      (Variables|/Script/Engine.CharacterMovementComponent|SetMaxWalkSpeed (Variables|Character|GetCharacterMovement) 6e+02)
      (Utilities|FlowControl|Delay (Variables|Default|GetThrowKnifeCooldown))
      (Variables|Default|SetLock false))))

(event EventStunned
  (bind _charactermovement (Variables|Character|GetCharacterMovement))
  (Variables|/Script/Engine.CharacterMovementComponent|SetMaxWalkSpeed _charactermovement 5e+01)
  (Utilities|FlowControl|Delay 5.0)
  (Variables|/Script/Engine.CharacterMovementComponent|SetMaxWalkSpeed _charactermovement 6e+02))

(event EventToggleAIFunctionality
  (params (Active :type Boolean))
  (Variables|Default|SetisActive Active)
  (Components|Movement|StopMovementImmediately (Variables|Character|GetCharacterMovement))
  (Class|NavMovementComponent|StopActiveMovement (Variables|Character|GetCharacterMovement)))

(event EventTick
  (params (DeltaSeconds :type Float%20%28single-precision%29))
  (if (Variables|Default|GetisActive)
    (CallFunction|CheckifinPlayerFOV)
    (if (Variables|Default|GetIsInPlayerView)
      (if (not (== (Variables|Default|GetRunningAway) (not (Variables|Default|GetVanishing))))
        (CallFunction|RunAway))
      (elif (not (Variables|Default|GetDeadBool))
        (if (Variables|Default|GetDealDamage)
          (Utilities|FlowControl|Delay 0.2)
          (CallFunction|DealDamageFunc (Variables|Default|GetPlayer))
          (else
            ;[1 1 1] Wait A Random Amount Of Time
            (if (not (Variables|Default|GetCanSeePlayer))
              (Utilities|FlowControl|Delay (Math|Random|RandomFloatinRange 2.0 4.0))
              ;[1 1 1] Move AI To A Random Location Within A Radius Of 4000 From Itself
              (if (Variables|Default|GetisActive)
                (AI|AIMoveTo self (.RandomLocation (AI|Navigation|GetRandomReachablePointinRadius (Transformation|GetActorLocation) 4e+03 0 0)) 0 5.0 true
                  (:then
                    (Variables|Default|SetIsMoving true)
                    (Utilities|FlowControl|Delay (Variables|Default|GetAmountOfTimeUntilDropGrenade))
                    (bind _outhit (Collision|LineTraceByChannel (Transformation|GetActorLocation) (* (Math|Vector|VectorDown) 5e+01) "TraceTypeQuery1" false 0 "None"))
                    (bind _returnvalue (Game|SpawnActorfromClass "/Game/Blueprints/Weapons/BP_A10_Grenade.BP_A10_Grenade_C" (Math|Transform|MakeTransform (.location _outhit) "0, 0, 0" "1.000000,1.000000,1.000000") "Undefined" 0 0))
                    (Utilities|FlowControl|Delay (Variables|Default|GetTimeUntilDropGrenadeExplode))
                    (Default|Explode _returnvalue))
                  (:OnSuccess
                    (Variables|Default|SetIsMoving false))))
              (elif (not (Variables|Default|GetLock))
                (Variables|Default|SetLock true)))))))))

(event EventSetSpeed
  (params (Speed :type Float%20%28double-precision%29))
  (Variables|/Script/Engine.CharacterMovementComponent|SetMaxWalkSpeed (Variables|Character|GetCharacterMovement) Speed))

(event EventFindPlayer
  (CallFunction|ChasePlayer (Game|Player|GetPlayerPawn 0)))

(event EventGetBPAudioManager
  (params (BP%20Audio%20Manager :type BP%20Audio%20Manager%20Object%20Reference))
  (Variables|Default|SetBP%20Audio%20Manager BP%20Audio%20Manager))

(event EventBeginPlay
  (bind _asbp_player_movement (Utilities|Casting|CastToBP_PlayerMovement (Game|GetPlayerCharacter 0)))
  (Variables|Default|SetPlayer _asbp_player_movement))

(fn ConstructionScript)

(fn DamageDeal
  (params (Damage :type Integer))
  (if (not (Variables|Default|GetDeadBool))
    (Variables|Default|SetHealth (- (Variables|Default|GetHealth) Damage))
    (if (<= (Variables|Default|GetHealth) 0.0)
      (CallFunction|Dead)
      (else
        (CallFunction|TookDamage)))))

(fn GetHealth
  (return (Variables|Default|GetHealth)))