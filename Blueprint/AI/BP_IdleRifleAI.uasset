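; Enemy rifle AI character that turns to face and shoots the player or tutorial player, with no movement logic of its own.
; Pawn sensing drives delayed firing and a retriggerable sight-memory timeout, while AI perception also turns it toward the player.
; Shots are line traces randomly offset by recoil, with audio and optional muzzle light; hitbox overlap enables per-tick melee damage.
; Death plays an animation and reports its tag to BP_InteriorEntranceManager.
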(event OnTargetPerceptionUpdated(AIPerception)
  (params (Actor :type Actor%20Object%20Reference) (Stimulus :type AI%20Stimulus%20Structure))
  (if (Variables|Default|GetisActive)
    (if (not (Variables|Default|GetDeadBool))
      (Development|PrintString "AI Heard Sound")
      (CallFunction|SeePlayer))))

(event OnSeePawn(PawnSensing)
  (params (Pawn :type Pawn%20Object%20Reference))
  (if (Variables|Default|GetisActive)
    _
    (elif (Variables|Default|GetCanSeePlayer)
      _
      (else
        (Utilities|FlowControl|Delay (Variables|Default|GetSeePlayerDelay)))))
  (CallFunction|ChasePlayer Pawn)
  (if (not (Variables|Default|GetDeadBool))
    (Utilities|FlowControl|Delay (Variables|Default|GetFireRate))
    (CallFunction|Shoot)))

(event OnComponentBeginOverlap(HitBox)
  (params (OverlappedComponent :type Primitive%20Component%20Object%20Reference) (OtherActor :type Actor%20Object%20Reference) (OtherComp :type Primitive%20Component%20Object%20Reference) (OtherBodyIndex :type Integer) (bFromSweep :type Boolean) (SweepResult :type Hit%20Result%20Structure%20%28by%20ref%29))
  ;[1 1 1] Collision
  (if (not (Variables|Default|GetDeadBool))
    (bind _asbp_player_movement (Utilities|Casting|CastToBP_PlayerMovement OtherActor))
    (if (Variables|/Script/ExtractShooter.PlayerMovement|GetDead _asbp_player_movement)
      (Variables|Default|SetDealMeleeDamage false)
      (elif (Collision|IsOverlappingActor (Variables|/Script/Engine.Character|GetMesh _asbp_player_movement) self :!class /Script/Engine.PrimitiveComponent)
        (Variables|Default|SetPlayer _asbp_player_movement)
        (Variables|Default|SetDealMeleeDamage true)))))

(event OnComponentEndOverlap(HitBox)
  (params (OverlappedComponent :type Primitive%20Component%20Object%20Reference) (OtherActor :type Actor%20Object%20Reference) (OtherComp :type Primitive%20Component%20Object%20Reference) (OtherBodyIndex :type Integer))
  ;[1 1 1] Collision
  (Utilities|Casting|CastToBP_PlayerMovement OtherActor)
  (Variables|Default|SetDealMeleeDamage false))

(event Custom|Dead
  ;[1 1 1] Dead
  (Development|PrintString "Dead")
  (Variables|Default|SetDeadBool true)
  (Components|Movement|StopMovementImmediately (Variables|Character|GetCharacterMovement))
  (Components|Animation|PlayAnimation (Variables|Character|GetMesh) "/Game/Assets/Models/Player/Dead/Falling_Forward_Death_Anim_mixamo_com.Falling_Forward_Death_Anim_mixamo_com" false)
  (bind _returnvalue (Actor|GetActorOfClass "/Game/Blueprints/UtilityItems/BP_InteriorEntranceManager.BP_InteriorEntranceManager_C"))
  (bind _asbp_interior_entrance_manager (Utilities|Casting|CastToBP_InteriorEntranceManager _returnvalue))
  (Default|SetDeadEnemiesFunc _asbp_interior_entrance_manager (Utilities|Array|Get(acopy) (Variables|Actor|GetTags self))))

(event Custom|DealDamageFunc
  (params (Player :type BP%20Player%20Movement%20Object%20Reference))
  ;[1 1 1] Dead Damage Func
  (if (Variables|/Script/ExtractShooter.PlayerMovement|GetDead Player)
    (Variables|Default|SetDealMeleeDamage false)
    (else
      (Development|PrintString "Enemy AI Hit Player")
      (Class|PlayerMovement|DealDamagetoPlayer Player (Variables|Default|GetDamage)))))

(event Custom|Shoot
  (bind _returnvalue (Transformation|GetActorLocation))
  (bind _damage (Variables|Default|GetDamage))
  (bind _weaponrecoil (Variables|Default|GetWeaponRecoil))
  (bind _returnvalue_2 (+ (.z _returnvalue) 6e+01))
  (if (== (Variables|Default|GetBP%20Audio%20Manager) 0) :!label _label
    (bind _returnvalue_3 (Actor|GetActorOfClass "/Game/Blueprints/Audio/BP_AudioManager.BP_AudioManager_C"))
    (Variables|Default|SetBP%20Audio%20Manager _returnvalue_3)
    (goto _label)
    (else
      ;[1 1 1] Shoot
      (Default|PlaySFXbyName (Variables|Default|GetBP%20Audio%20Manager) "AssaultRifleShoot" (Transformation|GetActorLocation))
      (bind _returnvalue_4 (Actor|GetActorOfClass "/Game/Blueprints/Player/BP_PlayerMovement.BP_PlayerMovement_C"))
      (Variables|Default|SetIsFiring true)
      (bind (_outhit _returnvalue_5) (Collision|LineTraceByChannel (Math|Vector|MakeVector (.x _returnvalue) (.y _returnvalue) _returnvalue_2) (Math|Vector|MakeVector (Math|Random|RandomFloatinRange (.x (Transformation|GetActorLocation _returnvalue_4)) (+ (.x (Transformation|GetActorLocation _returnvalue_4)) _weaponrecoil)) (Math|Random|RandomFloatinRange (.y (Transformation|GetActorLocation _returnvalue_4)) (+ (.y (Transformation|GetActorLocation _returnvalue_4)) _weaponrecoil)) (Math|Random|RandomFloatinRange (.z (Transformation|GetActorLocation _returnvalue_4)) (+ (.z (Transformation|GetActorLocation _returnvalue_4)) _weaponrecoil))) "TraceTypeQuery1" true (Variables|Default|GetActors%20to%20Ignore) "None"))
      (CallFunction|FlashLights)
      (Rendering|Debug|DrawDebugLine (Math|Vector|MakeVector (.x _returnvalue) (.y _returnvalue) _returnvalue_2) (Math|Vector|MakeVector 0.0 0.0 0.0) "(R=0.000000,G=0.342474,B=1.000000,A=1.000000)" 2.0 1.0)
      (if _returnvalue_5
        (Development|PrintString (Utilities|GetDisplayName (.HitActor (Collision|BreakHitResult _outhit))))
        (bind _asbp_player_movement (Utilities|Casting|CastToBP_PlayerMovement (.HitActor (Collision|BreakHitResult _outhit)))
          (:then
            (Class|PlayerMovement|DealDamagetoPlayer _asbp_player_movement _damage)
            (Development|PrintString "WORKED"))
          (:CastFailed
            (bind _asbp_player_movement_tutorial (Utilities|Casting|CastToBP_PlayerMovementTutorial (.HitActor (Collision|BreakHitResult _outhit))))
            (Class|PlayerMovement|DealDamagetoPlayer _asbp_player_movement_tutorial _damage)))))))

(event Custom|FlashLights
  (bind _asbp_game_instance (Utilities|Casting|CastToBP_GameInstance (Game|GetGameInstance)))
  (if (Variables|/Game/Blueprints/BP_GameInstance.BP_GameInstance_C|GetShowMuzzleFlash _asbp_game_instance)
    (Rendering|SetVisibility (Variables|Default|GetPointLight) true false)
    (Utilities|FlowControl|Delay 0.2)
    (Rendering|SetVisibility (Variables|Default|GetPointLight) false false)))

(event Custom|Chase%20Player
  (params (Pawn :type Pawn%20Object%20Reference))
  (if (Variables|Default|GetisActive)
    (if (not (Variables|Default|GetDeadBool))
      (Utilities|Casting|CastToBP_PlayerMovement Pawn
        (:then
          (Utilities|FlowControl|Sequence
            (:then_0
              (CallFunction|SeePlayer))
            (:then_1
              ;[1 1 1] Can't See Player
              (Utilities|FlowControl|RetriggerableDelay (Variables|Default|GetMemory) :!label _label)
              (Variables|Default|SetCanSeePlayer false)
              (Variables|Default|SetIsFiring false))))
        (:CastFailed
          (bind _asbp_player_movement_tutorial (Utilities|Casting|CastToBP_PlayerMovementTutorial Pawn))
          (Utilities|FlowControl|Sequence
            (:then_0
              ;[1 1 1] Shoot Player On Sight
              (Variables|Default|SetCanSeePlayer true)
              (Transformation|SetActorRotation (Math|Rotator|FindLookatRotation (Transformation|GetActorLocation) (Transformation|GetActorLocation _asbp_player_movement_tutorial)))
              (Utilities|FlowControl|Delay (Variables|Default|GetFireRate))
              (CallFunction|Shoot))
            (:then_1
              (goto _label))))))))

(event Custom|See%20Player
  (bind _returnvalue (Actor|GetActorOfClass "/Game/Blueprints/Player/BP_PlayerMovement.BP_PlayerMovement_C"))
  (Variables|Default|SetCanSeePlayer true)
  (Transformation|SetActorRotation (Math|Rotator|FindLookatRotation (Transformation|GetActorLocation) (Transformation|GetActorLocation _returnvalue))))

(event EventBeginPlay
  ;[1 1 1] Bind Weapon Mesh To Hand
  (Transformation|AttachComponentToComponent (Variables|Default|GetA90%20Rifle) (Variables|Character|GetMesh) "RightHandSocket" "SnapToTarget" "SnapToTarget" "KeepRelative" true)
  (bind _outactors (Actor|GetAllActorswithTag "Ignore"))
  (Variables|Default|SetActors%20to%20Ignore _outactors))

(event EventToggleAIFunctionality
  (params (Active :type Boolean))
  (Variables|Default|SetisActive Active)
  (Components|Movement|StopMovementImmediately (Variables|Character|GetCharacterMovement))
  (Class|NavMovementComponent|StopActiveMovement (Variables|Character|GetCharacterMovement)))

(event EventTick
  (params (DeltaSeconds :type Float%20%28single-precision%29))
  ;[1 1 1] Dead Damage To Player
  (if (Variables|Default|GetisActive)
    (if (not (Variables|Default|GetDeadBool))
      (if (Variables|Default|GetDealMeleeDamage)
        (CallFunction|DealDamageFunc (Variables|Default|GetPlayer))))))

(event EventFindPlayer
  (CallFunction|ChasePlayer (Game|Player|GetPlayerPawn 0)))

(event EventGetBPAudioManager
  (params (BP%20Audio%20Manager :type BP%20Audio%20Manager%20Object%20Reference))
  (Variables|Default|SetBP%20Audio%20Manager BP%20Audio%20Manager))

(fn ConstructionScript)

(fn DamageDeal
  (params (Damage :type Integer))
  (if (not (Variables|Default|GetDeadBool))
    (Variables|Default|SetHealth (- (Variables|Default|GetHealth) Damage))
    (if (<= (Variables|Default|GetHealth) 0.0)
      (CallFunction|Dead))))

(fn GetHealth
  (return (Variables|Default|GetHealth)))