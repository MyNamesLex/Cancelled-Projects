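; Level audio manager actor that plays background music and named sound effects, and makes player sounds audible to AI.
; On BeginPlay it reads volumes from the GameInstance, starts BGM there, and hands itself to exit, AI and trap interface actors plus the player.
; Name-matched branch chains play SFX in 2D or at a location, with selected sounds triggering MakeNoise.
; It can also fade music out before opening the next level.
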(event Custom|Play%20BGM%20Music
  (bind _asbp_game_instance (Utilities|Casting|CastToBP_GameInstance (Game|GetGameInstance))
    (:then
      (Default|PlayBGMMusic _asbp_game_instance (Variables|Default|GetCurrentBGM) "/Game/Blueprints/Audio/BP_SoundConcurrency.BP_SoundConcurrency" (Variables|Default|GetBGMFadeInTime)))
    (:CastFailed
      (Development|PrintString "FAILED CAST TO BP GAME INSTANCE BP AUDIO MANAGER"))))

(event Custom|Stop%20Music
  (bind _asbp_game_instance (Utilities|Casting|CastToBP_GameInstance (Game|GetGameInstance)))
  (Default|StopBGMMusic _asbp_game_instance))

(event Custom|ChangePlayingBGMVolume
  (bind _asbp_game_instance (Utilities|Casting|CastToBP_GameInstance (Game|GetGameInstance)))
  (Audio|Components|Audio|Stop (Variables|/Game/Blueprints/BP_GameInstance.BP_GameInstance_C|GetBGM%20Playing _asbp_game_instance))
  (Variables|/Game/Blueprints/BP_GameInstance.BP_GameInstance_C|SetBGM%20Playing _asbp_game_instance 0)
  (CallFunction|PlayBGMMusic))

(event Custom|PlaySFXByName
  (params (AudioName :type String) (Location :type Vector))
  (bind _sfxvolume (Variables|Default|GetSFXVolume))
  (bind _sfxvolume_2 (Variables|Default|GetSFXVolume))
  (if (Utilities|Enum|Equal(Enum) AudioName "ChargePistolShoot")
    (bind _returnvalue (Audio|SpawnSoundatLocation (Variables|Default|GetChargePistolShoot) Location "0, 0, 0" _sfxvolume_2 1.0 0.0 "/Game/Blueprints/Audio/BP_SoundAttenuation.BP_SoundAttenuation" "/Game/Blueprints/Audio/BP_SoundConcurrency.BP_SoundConcurrency" false))
    (Variables|Default|SetChargePistolShootSFXPlaying _returnvalue)
    (bind _asbp_player_movement (Utilities|Casting|CastToBP_PlayerMovement (Game|GetPlayerCharacter 0) :!label _label))
    (if (or (Variables|/Script/ExtractShooter.PlayerMovement|GetisShootingPistol _asbp_player_movement) (Variables|/Script/ExtractShooter.PlayerMovement|GetisShootingRifle _asbp_player_movement))
      (Class|Actor|MakeNoise _asbp_player_movement 1.0 _asbp_player_movement (Transformation|GetActorLocation _asbp_player_movement) (Variables|Default|GetMaxAIHearingRange) "None")
      (Development|PrintString "MAKE NOISE PLAYER SHOOTING"))
    (elif (Utilities|Enum|Equal(Enum) AudioName "PistolShoot")
      (bind _returnvalue_2 (Audio|SpawnSoundatLocation (Variables|Default|GetPistolShoot) Location "0, 0, 0" _sfxvolume_2 1.0 0.0 "/Game/Blueprints/Audio/BP_SoundAttenuation.BP_SoundAttenuation" "/Game/Blueprints/Audio/BP_SoundConcurrency.BP_SoundConcurrency" false))
      (Variables|Default|SetPistolShootSFXPlaying _returnvalue_2)
      (goto _label)
      (elif (Utilities|Enum|Equal(Enum) AudioName "PistolReload")
        (bind _returnvalue_3 (Audio|SpawnSoundatLocation (Variables|Default|GetPistolReload) Location "0, 0, 0" _sfxvolume_2 1.0 0.0 "/Game/Blueprints/Audio/BP_SoundAttenuation.BP_SoundAttenuation" "/Game/Blueprints/Audio/BP_SoundConcurrency.BP_SoundConcurrency" false))
        (Variables|Default|SetPistolReloadSFXPlaying _returnvalue_3)
        (elif (Utilities|Enum|Equal(Enum) AudioName "AssaultRifleShoot")
          (bind _returnvalue_4 (Audio|SpawnSoundatLocation (Variables|Default|GetAssaultRifleShoot) Location "0, 0, 0" _sfxvolume_2 1.0 0.0 "/Game/Blueprints/Audio/BP_SoundAttenuation.BP_SoundAttenuation" "/Game/Blueprints/Audio/BP_SoundConcurrency.BP_SoundConcurrency" false))
          (Variables|Default|SetAssaultRifleShootSFXPlaying _returnvalue_4)
          (goto _label)
          (elif (Utilities|Enum|Equal(Enum) AudioName "AssaultRifleStopShooting")
            (bind _returnvalue_5 (Audio|SpawnSoundatLocation (Variables|Default|GetStopShootingAssaultRifle) Location "0, 0, 0" _sfxvolume 1.0 0.0 "/Game/Blueprints/Audio/BP_SoundAttenuation.BP_SoundAttenuation" "/Game/Blueprints/Audio/BP_SoundConcurrency.BP_SoundConcurrency" false))
            (Variables|Default|SetStopShootingAssaultRifleSFXPlaying _returnvalue_5)
            (elif (Utilities|Enum|Equal(Enum) AudioName "AssaultRifleReload")
              (bind _returnvalue_6 (Audio|SpawnSoundatLocation (Variables|Default|GetAssaultRifleReload) Location "0, 0, 0" _sfxvolume 1.0 0.0 "/Game/Blueprints/Audio/BP_SoundAttenuation.BP_SoundAttenuation" "/Game/Blueprints/Audio/BP_SoundConcurrency.BP_SoundConcurrency" false))
              (Variables|Default|SetAssaultRifleReloadSFXPlaying _returnvalue_6)
              (elif (Utilities|Enum|Equal(Enum) AudioName "SniperShoot")
                (bind _returnvalue_7 (Audio|SpawnSoundatLocation (Variables|Default|GetSniperShoot) Location "0, 0, 0" _sfxvolume 1.0 0.0 "/Game/Blueprints/Audio/BP_SoundAttenuation.BP_SoundAttenuation" "/Game/Blueprints/Audio/BP_SoundConcurrency.BP_SoundConcurrency" false))
                (Variables|Default|SetSniperShootSFXPlaying _returnvalue_7)
                (goto _label)
                (elif (Utilities|Enum|Equal(Enum) AudioName "SniperReload")
                  (bind _returnvalue_8 (Audio|SpawnSoundatLocation (Variables|Default|GetSniperReload) Location "0, 0, 0" _sfxvolume 1.0 0.0 "/Game/Blueprints/Audio/BP_SoundAttenuation.BP_SoundAttenuation" "/Game/Blueprints/Audio/BP_SoundConcurrency.BP_SoundConcurrency" false))
                  (Variables|Default|SetSniperReloadSFXPlaying _returnvalue_8)
                  (elif (Utilities|Enum|Equal(Enum) AudioName "ShotgunShoot")
                    (bind _returnvalue_9 (Audio|SpawnSoundatLocation (Variables|Default|GetShotgunShoot) Location "0, 0, 0" _sfxvolume 1.0 0.0 "/Game/Blueprints/Audio/BP_SoundAttenuation.BP_SoundAttenuation" "/Game/Blueprints/Audio/BP_SoundConcurrency.BP_SoundConcurrency" false))
                    (Variables|Default|SetShotgunShootSFXPlaying _returnvalue_9)
                    (goto _label)
                    (elif (Utilities|Enum|Equal(Enum) AudioName "ShotgunReload")
                      (bind _returnvalue_10 (Audio|SpawnSoundatLocation (Variables|Default|GetShotgunReload) Location "0, 0, 0" _sfxvolume 1.0 0.0 "/Game/Blueprints/Audio/BP_SoundAttenuation.BP_SoundAttenuation" "/Game/Blueprints/Audio/BP_SoundConcurrency.BP_SoundConcurrency" false))
                      (Variables|Default|SetShotgunReloadSFXPlaying _returnvalue_10)
                      (elif (Utilities|Enum|Equal(Enum) AudioName "OutOfAmmoSFX")
                        (bind _returnvalue_11 (Audio|SpawnSoundatLocation (Variables|Default|GetOutOfAmmoSFX) Location "0, 0, 0" _sfxvolume 1.0 0.0 "/Game/Blueprints/Audio/BP_SoundAttenuation.BP_SoundAttenuation" "/Game/Blueprints/Audio/BP_SoundConcurrency.BP_SoundConcurrency" false))
                        (Variables|Default|SetOutOfAmmoSFXPlaying _returnvalue_11)
                        (elif (Utilities|Enum|Equal(Enum) AudioName "Jump")
                          (bind _returnvalue_12 (Audio|SpawnSoundatLocation (Variables|Default|GetJump) Location "0, 0, 0" _sfxvolume 1.0 0.0 "/Game/Blueprints/Audio/BP_SoundAttenuation.BP_SoundAttenuation" "/Game/Blueprints/Audio/BP_SoundConcurrency.BP_SoundConcurrency" false))
                          (Variables|Default|SetJumpSFXPlaying _returnvalue_12)
                          (elif (Utilities|Enum|Equal(Enum) AudioName "Dead")
                            (bind _returnvalue_13 (Audio|SpawnSoundatLocation (Variables|Default|GetDead) Location "0, 0, 0" _sfxvolume 1.0 0.0 "/Game/Blueprints/Audio/BP_SoundAttenuation.BP_SoundAttenuation" "/Game/Blueprints/Audio/BP_SoundConcurrency.BP_SoundConcurrency" false))
                            (Variables|Default|SetDeadSFXPlaying _returnvalue_13)
                            (elif (Utilities|Enum|Equal(Enum) AudioName "TookDamage")
                              (bind _returnvalue_14 (Audio|SpawnSoundatLocation (Variables|Default|GetTookDamage) Location "0, 0, 0" _sfxvolume 1.0 0.0 "/Game/Blueprints/Audio/BP_SoundAttenuation.BP_SoundAttenuation" "/Game/Blueprints/Audio/BP_SoundConcurrency.BP_SoundConcurrency" false))
                              (Variables|Default|SetTookDamageSFXPlaying _returnvalue_14)
                              (elif (Utilities|Enum|Equal(Enum) AudioName "PickupItem")
                                (bind _returnvalue_15 (Audio|SpawnSoundatLocation (Variables|Default|GetPickupItem) Location "0, 0, 0" _sfxvolume 1.0 0.0 "/Game/Blueprints/Audio/BP_SoundAttenuation.BP_SoundAttenuation" "/Game/Blueprints/Audio/BP_SoundConcurrency.BP_SoundConcurrency" false))
                                (Variables|Default|SetPickupItemSFXPlaying _returnvalue_15)
                                (elif (Utilities|Enum|Equal(Enum) AudioName "PickupWeapon")
                                  (bind _returnvalue_16 (Audio|SpawnSoundatLocation (Variables|Default|GetPickupWeapon) Location "0, 0, 0" _sfxvolume 1.0 0.0 "/Game/Blueprints/Audio/BP_SoundAttenuation.BP_SoundAttenuation" "/Game/Blueprints/Audio/BP_SoundConcurrency.BP_SoundConcurrency" false))
                                  (Variables|Default|SetPickupWeaponSFXPlaying _returnvalue_16)
                                  (elif (Utilities|Enum|Equal(Enum) AudioName "Explosion")
                                    (bind _returnvalue_17 (Audio|SpawnSoundatLocation (Variables|Default|GetExplosion) Location "0, 0, 0" _sfxvolume 1.0 0.0 "/Game/Blueprints/Audio/BP_SoundAttenuation.BP_SoundAttenuation" "/Game/Blueprints/Audio/BP_SoundConcurrency.BP_SoundConcurrency" false))
                                    (Variables|Default|SetExplosionSFXPlaying _returnvalue_17)
                                    (elif (Utilities|Enum|Equal(Enum) AudioName "SnaggedBarbedWire")
                                      (bind _returnvalue_18 (Audio|SpawnSoundatLocation (Variables|Default|GetSnaggedBarbedWire) Location "0, 0, 0" _sfxvolume 1.0 0.0 "/Game/Blueprints/Audio/BP_SoundAttenuation.BP_SoundAttenuation" "/Game/Blueprints/Audio/BP_SoundConcurrency.BP_SoundConcurrency" false))
                                      (Variables|Default|SetSnaggedBarbedWireSFXPlaying _returnvalue_18)
                                      (elif (Utilities|Enum|Equal(Enum) AudioName "RingingEars")
                                        (bind _returnvalue_19 (Audio|SpawnSoundatLocation (Variables|Default|GetRingingEars) Location "0, 0, 0" _sfxvolume 1.0 0.0 "/Game/Blueprints/Audio/BP_SoundAttenuation.BP_SoundAttenuation" "/Game/Blueprints/Audio/BP_SoundConcurrency.BP_SoundConcurrency" false))
                                        (Variables|Default|SetRingingEarsSFXPlaying _returnvalue_19)
                                        (elif (Utilities|Enum|Equal(Enum) AudioName "Melee")
                                          (bind _returnvalue_20 (Audio|SpawnSoundatLocation (Variables|Default|GetMelee) Location "0, 0, 0" _sfxvolume 1.0 0.0 "/Game/Blueprints/Audio/BP_SoundAttenuation.BP_SoundAttenuation" "/Game/Blueprints/Audio/BP_SoundConcurrency.BP_SoundConcurrency" false))
                                          (Variables|Default|SetMeleeSFXPlaying _returnvalue_20)
                                          (elif (Utilities|Enum|Equal(Enum) AudioName "UnscopeADS")
                                            (bind _returnvalue_21 (Audio|SpawnSoundatLocation (Variables|Default|GetUnscopeADS) Location "0, 0, 0" _sfxvolume 1.0 0.0 "/Game/Blueprints/Audio/BP_SoundAttenuation.BP_SoundAttenuation" "/Game/Blueprints/Audio/BP_SoundConcurrency.BP_SoundConcurrency" false))
                                            (Variables|Default|SetUnscopeSFXPlaying _returnvalue_21)
                                            (elif (Utilities|Enum|Equal(Enum) AudioName "ADS")
                                              (bind _returnvalue_22 (Audio|SpawnSoundatLocation (Variables|Default|GetADS) Location "0, 0, 0" _sfxvolume 1.0 0.0 "/Game/Blueprints/Audio/BP_SoundAttenuation.BP_SoundAttenuation" "/Game/Blueprints/Audio/BP_SoundConcurrency.BP_SoundConcurrency" false))
                                              (Variables|Default|SetADSSFXPlaying _returnvalue_22)
                                              (elif (Utilities|Enum|Equal(Enum) AudioName "CanDash")
                                                (bind _returnvalue_23 (Audio|SpawnSoundatLocation (Variables|Default|GetCanDash) Location "0, 0, 0" _sfxvolume 1.0 0.0 "/Game/Blueprints/Audio/BP_SoundAttenuation.BP_SoundAttenuation" "/Game/Blueprints/Audio/BP_SoundConcurrency.BP_SoundConcurrency" false))
                                                (Variables|Default|SetCanDashSFXPlaying _returnvalue_23)
                                                (goto _label)
                                                (elif (Utilities|Enum|Equal(Enum) AudioName "Click")
                                                  (bind _returnvalue_24 (Audio|SpawnSoundatLocation (Variables|Default|GetClick) Location "0, 0, 0" _sfxvolume 1.0 0.0 "/Game/Blueprints/Audio/BP_SoundAttenuation.BP_SoundAttenuation" "/Game/Blueprints/Audio/BP_SoundConcurrency.BP_SoundConcurrency" false))
                                                  (Variables|Default|SetClickSFXPlaying _returnvalue_24)
                                                  (else
                                                    (Development|PrintString "BP AUDIO MANAGER, AUDIO DID NOT PLAY - AUDIO NAME = ")
                                                    (if (Utilities|Enum|Equal(Enum) AudioName "")
                                                      (Development|PrintString "AUDIO NAME IS NULL")
                                                      (else
                                                        (Development|PrintString AudioName)))))))))))))))))))))))))))))

(event Custom|PlaySFXByName2D
  (params (SFXName :type String))
  (if (Utilities|Enum|Equal(Enum) SFXName "ChargePistolShoot")
    (Audio|PlaySound2D (Variables|Default|GetChargePistolShoot) (Variables|Default|GetSFXVolume) 1.0 0.0 "/Game/Blueprints/Audio/BP_SoundConcurrency.BP_SoundConcurrency" (Game|GetPlayerController 0) false)
    (bind _asbp_player_movement (Utilities|Casting|CastToBP_PlayerMovement (Game|GetPlayerCharacter 0) :!label _label))
    (Class|Actor|MakeNoise _asbp_player_movement 1.0 _asbp_player_movement (Transformation|GetActorLocation _asbp_player_movement) (Variables|Default|GetMaxAIHearingRange) "None")
    (Development|PrintString "Player Made Noise")
    (elif (Utilities|Enum|Equal(Enum) SFXName "PistolShoot")
      (Audio|PlaySound2D (Variables|Default|GetPistolShoot) (Variables|Default|GetSFXVolume) 1.0 0.0 "/Game/Blueprints/Audio/BP_SoundConcurrency.BP_SoundConcurrency" (Game|GetPlayerController 0) false)
      (goto _label)
      (elif (Utilities|Enum|Equal(Enum) SFXName "PistolReload")
        (Audio|PlaySound2D (Variables|Default|GetPistolReload) (Variables|Default|GetSFXVolume) 1.0 0.0 "/Game/Blueprints/Audio/BP_SoundConcurrency.BP_SoundConcurrency" (Game|GetPlayerController 0) false)
        (goto _label)
        (elif (Utilities|Enum|Equal(Enum) SFXName "AssaultRifleShoot")
          (Audio|PlaySound2D (Variables|Default|GetAssaultRifleShoot) (Variables|Default|GetSFXVolume) 1.0 0.0 "/Game/Blueprints/Audio/BP_SoundConcurrency.BP_SoundConcurrency" (Game|GetPlayerController 0) false)
          (goto _label)
          (elif (Utilities|Enum|Equal(Enum) SFXName "AssaultRifleStopShooting")
            (Audio|PlaySound2D (Variables|Default|GetStopShootingAssaultRifle) (Variables|Default|GetSFXVolume) 1.0 0.0 "/Game/Blueprints/Audio/BP_SoundConcurrency.BP_SoundConcurrency" (Game|GetPlayerController 0) false)
            (goto _label)
            (elif (Utilities|Enum|Equal(Enum) SFXName "AssaultRifleReload")
              (Audio|PlaySound2D (Variables|Default|GetAssaultRifleReload) (Variables|Default|GetSFXVolume) 1.0 0.0 "/Game/Blueprints/Audio/BP_SoundConcurrency.BP_SoundConcurrency" (Game|GetPlayerController 0) false)
              (goto _label)
              (elif (Utilities|Enum|Equal(Enum) SFXName "SniperShoot")
                (Audio|PlaySound2D (Variables|Default|GetSniperShoot) (Variables|Default|GetSFXVolume) 1.0 0.0 "/Game/Blueprints/Audio/BP_SoundConcurrency.BP_SoundConcurrency" (Game|GetPlayerController 0) false)
                (goto _label)
                (elif (Utilities|Enum|Equal(Enum) SFXName "SniperReload")
                  (Audio|PlaySound2D (Variables|Default|GetSniperReload) (Variables|Default|GetSFXVolume) 1.0 0.0 "/Game/Blueprints/Audio/BP_SoundConcurrency.BP_SoundConcurrency" (Game|GetPlayerController 0) false)
                  (goto _label)
                  (elif (Utilities|Enum|Equal(Enum) SFXName "ShotgunShoot")
                    (Audio|PlaySound2D (Variables|Default|GetShotgunShoot) (Variables|Default|GetSFXVolume) 1.0 0.0 "/Game/Blueprints/Audio/BP_SoundConcurrency.BP_SoundConcurrency" (Game|GetPlayerController 0) false)
                    (goto _label)
                    (elif (Utilities|Enum|Equal(Enum) SFXName "ShotgunReload")
                      (Audio|PlaySound2D (Variables|Default|GetShotgunReload) (Variables|Default|GetSFXVolume) 1.0 0.0 "/Game/Blueprints/Audio/BP_SoundConcurrency.BP_SoundConcurrency" (Game|GetPlayerController 0) false)
                      (goto _label)
                      (elif (Utilities|Enum|Equal(Enum) SFXName "OutOfAmmoSFX")
                        (Audio|PlaySound2D (Variables|Default|GetOutOfAmmoSFX) (Variables|Default|GetSFXVolume) 1.0 0.0 "/Game/Blueprints/Audio/BP_SoundConcurrency.BP_SoundConcurrency" (Game|GetPlayerController 0) false)
                        (goto _label)
                        (elif (Utilities|Enum|Equal(Enum) SFXName "Jump")
                          (Audio|PlaySound2D (Variables|Default|GetJump) (Variables|Default|GetSFXVolume) 1.0 0.0 "/Game/Blueprints/Audio/BP_SoundConcurrency.BP_SoundConcurrency" (Game|GetPlayerController 0) false)
                          (goto _label)
                          (elif (Utilities|Enum|Equal(Enum) SFXName "Dead")
                            (Audio|PlaySound2D (Variables|Default|GetDead) (Variables|Default|GetSFXVolume) 1.0 0.0 "/Game/Blueprints/Audio/BP_SoundConcurrency.BP_SoundConcurrency" (Game|GetPlayerController 0) false)
                            (goto _label)
                            (elif (Utilities|Enum|Equal(Enum) SFXName "TookDamage")
                              (Audio|PlaySound2D (Variables|Default|GetTookDamage) (Variables|Default|GetSFXVolume) 1.0 0.0 "/Game/Blueprints/Audio/BP_SoundConcurrency.BP_SoundConcurrency" (Game|GetPlayerController 0) false)
                              (goto _label)
                              (elif (Utilities|Enum|Equal(Enum) SFXName "PickupItem")
                                (Audio|PlaySound2D (Variables|Default|GetPickupItem) (Variables|Default|GetSFXVolume) 1.0 0.0 "/Game/Blueprints/Audio/BP_SoundConcurrency.BP_SoundConcurrency" (Game|GetPlayerController 0) false)
                                (goto _label)
                                (elif (Utilities|Enum|Equal(Enum) SFXName "PickupWeapon")
                                  (Audio|PlaySound2D (Variables|Default|GetPickupWeapon) (Variables|Default|GetSFXVolume) 1.0 0.0 "/Game/Blueprints/Audio/BP_SoundConcurrency.BP_SoundConcurrency" (Game|GetPlayerController 0) false)
                                  (goto _label)
                                  (elif (Utilities|Enum|Equal(Enum) SFXName "Explosion")
                                    (Audio|PlaySound2D (Variables|Default|GetExplosion) (Variables|Default|GetSFXVolume) 1.0 0.0 "/Game/Blueprints/Audio/BP_SoundConcurrency.BP_SoundConcurrency" 0 false)
                                    (goto _label)
                                    (elif (Utilities|Enum|Equal(Enum) SFXName "SnaggedBarbedWire")
                                      (Audio|PlaySound2D (Variables|Default|GetSnaggedBarbedWire) (Variables|Default|GetSFXVolume) 1.0 0.0 "/Game/Blueprints/Audio/BP_SoundConcurrency.BP_SoundConcurrency" (Game|GetPlayerController 0) false)
                                      (goto _label)
                                      (elif (Utilities|Enum|Equal(Enum) SFXName "RingingEars")
                                        (Audio|PlaySound2D (Variables|Default|GetRingingEars) (Variables|Default|GetSFXVolume) 1.0 0.0 "/Game/Blueprints/Audio/BP_SoundConcurrency.BP_SoundConcurrency" (Game|GetPlayerController 0) false)
                                        (goto _label)
                                        (elif (Utilities|Enum|Equal(Enum) SFXName "Melee")
                                          (Audio|PlaySound2D (Variables|Default|GetMelee) (Variables|Default|GetSFXVolume) 1.0 0.0 "/Game/Blueprints/Audio/BP_SoundConcurrency.BP_SoundConcurrency" (Game|GetPlayerController 0) false)
                                          (Development|PrintString "SILENT SOUND AI NOT HEAR" :!label _label_2)
                                          (elif (Utilities|Enum|Equal(Enum) SFXName "UnscopeADS")
                                            (Audio|PlaySound2D (Variables|Default|GetUnscopeADS) (Variables|Default|GetSFXVolume) 1.0 0.0 "/Game/Blueprints/Audio/BP_SoundConcurrency.BP_SoundConcurrency" (Game|GetPlayerController 0) false)
                                            (goto _label_2)
                                            (elif (Utilities|Enum|Equal(Enum) SFXName "ADS")
                                              (Audio|PlaySound2D (Variables|Default|GetADS) (Variables|Default|GetSFXVolume) 1.0 0.0 "/Game/Blueprints/Audio/BP_SoundConcurrency.BP_SoundConcurrency" (Game|GetPlayerController 0) false)
                                              (goto _label_2)
                                              (elif (Utilities|Enum|Equal(Enum) SFXName "CanDash")
                                                (Audio|PlaySound2D (Variables|Default|GetCanDash) (Variables|Default|GetSFXVolume) 1.0 0.0 "/Game/Blueprints/Audio/BP_SoundConcurrency.BP_SoundConcurrency" (Game|GetPlayerController 0) false)
                                                (goto _label_2)
                                                (elif (Utilities|Enum|Equal(Enum) SFXName "Click")
                                                  (Audio|PlaySound2D (Variables|Default|GetClick) (Variables|Default|GetSFXVolume) 1.0 0.0 "/Game/Blueprints/Audio/BP_SoundConcurrency.BP_SoundConcurrency" (Game|GetPlayerController 0) false)
                                                  (goto _label_2)
                                                  (else
                                                    (Development|PrintString "BP AUDIO MANAGER, AUDIO DID NOT PLAY - AUDIO NAME = ")
                                                    (if (Utilities|Enum|Equal(Enum) SFXName "")
                                                      (Development|PrintString "AUDIO NAME IS NULL")
                                                      (else
                                                        (Development|PrintString "Hello")))))))))))))))))))))))))))))

(event Custom|FadeOutBGMLoadNextLevel
  (params (FadeOutTime :type Float%20%28double-precision%29) (NextLevelName :type Name))
  (bind _asbp_game_instance (Utilities|Casting|CastToBP_GameInstance (Game|GetGameInstance)))
  (Audio|Components|Audio|FadeOut (Variables|/Game/Blueprints/BP_GameInstance.BP_GameInstance_C|GetBGM%20Playing _asbp_game_instance) FadeOutTime 0.0 "Linear" :!class /Script/Engine.AudioComponent)
  (if (Audio|Components|Audio|IsPlaying (Variables|/Game/Blueprints/BP_GameInstance.BP_GameInstance_C|GetBGM%20Playing _asbp_game_instance)) :!label _label
    (Utilities|FlowControl|DelayUntilNextTick)
    (goto _label)
    (else
      (Default|StopBGMMusic _asbp_game_instance)
      (Variables|/Game/Blueprints/BP_GameInstance.BP_GameInstance_C|SetBGM%20Playing _asbp_game_instance 0)
      (Game|OpenLevel(byName) NextLevelName))))

(event EventBeginPlay
  (bind _returnvalue (Game|GetPlayerCharacter 0))
  (bind _asbp_game_instance (Utilities|Casting|CastToBP_GameInstance (Game|GetGameInstance)))
  (Variables|Default|SetSFXVolume (Variables|/Game/Blueprints/BP_GameInstance.BP_GameInstance_C|GetSFXVolume _asbp_game_instance))
  (Variables|Default|SetBGMVolume (Variables|/Game/Blueprints/BP_GameInstance.BP_GameInstance_C|GetBGMVolume _asbp_game_instance))
  (CallFunction|PlayBGMMusic)
  (bind _outactors (Actor|GetAllActorswithInterface "/Game/Blueprints/UtilityItems/BP_ExitInterface.BP_ExitInterface_C"))
  (for _array_element _outactors
    (Class|BPExitInterface|GetBPAudioManager(Message) _array_element self))
  (bind _outactors_2 (Actor|GetAllActorswithInterface "/Game/Blueprints/AI/BP_AIInterface.BP_AIInterface_C"))
  (for _array_element_2 _outactors_2
    (Class|BPAIInterface|GetBPAudioManager(Message) _array_element_2 self))
  (bind _outactors_3 (Actor|GetAllActorswithInterface "/Game/Blueprints/Traps/BP_TrapInterface.BP_TrapInterface_C"))
  (for _array_element_3 _outactors_3
    (Class|BPTrapInterface|GetBPAudioManager(Message) _array_element_3 self))
  (bind _asbp_player_movement (Utilities|Casting|CastToBP_PlayerMovement _returnvalue)
    (:then
      (Variables|/Game/Blueprints/Player/BP_PlayerMovement.BP_PlayerMovement_C|SetBP%20Audio%20Manager _asbp_player_movement self))
    (:CastFailed
      (bind _asbp_player_movement_tutorial (Utilities|Casting|CastToBP_PlayerMovementTutorial _returnvalue)
        (:then
          (Variables|/Game/Blueprints/Tutorial/BP_PlayerMovementTutorial.BP_PlayerMovementTutorial_C|SetBP%20Audio%20Manager _asbp_player_movement_tutorial self)
          (Development|PrintString "BP PLAYER TUTORIAL AUDIO MANAGER SET"))
        (:CastFailed
          (Development|PrintString "CAST TO BP PLAYERMOVEMENT AND BP PLAYER MOVEMENT TUTORIAL FAILED BP AUDIOMANAGER"))))))

(event Collision|EventActorBeginOverlap
  (params (OtherActor :type Actor%20Object%20Reference)))

(event EventTick
  (params (DeltaSeconds :type Float%20%28single-precision%29)))

(fn ConstructionScript)