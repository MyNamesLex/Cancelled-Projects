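; BP_BarbedWire is a trap that slows the player and AI that overlap it and damages the player while caught.
; Overlap start cuts movement speed, flags the player as stunned and plays a snag sound; overlap end resets speeds to fixed values.
; Tick uses a Delay as a repeating timer, dealing damage with sound while contact persists.
; AI speed goes through BP_AIInterface, and the audio manager is supplied via GetBPAudioManager.
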(event OnComponentBeginOverlap(BarbedWireFull)
  (params (OverlappedComponent :type Primitive%20Component%20Object%20Reference) (OtherActor :type Actor%20Object%20Reference) (OtherComp :type Primitive%20Component%20Object%20Reference) (OtherBodyIndex :type Integer) (bFromSweep :type Boolean) (SweepResult :type Hit%20Result%20Structure%20%28by%20ref%29))
  (bind _asbp_player_movement (Utilities|Casting|CastToBP_PlayerMovement OtherActor)
    (:then
      (Variables|Default|SetPlayer _asbp_player_movement)
      (Variables|Default|SetPlayerColliding true)
      (Variables|/Script/Engine.CharacterMovementComponent|SetMaxWalkSpeed (Variables|/Script/Engine.Character|GetCharacterMovement _asbp_player_movement) 1.5e+02)
      (Variables|/Script/ExtractShooter.PlayerMovement|SetStunned _asbp_player_movement true)
      (Default|PlaySFXbyName (Variables|Default|GetBP%20Audio%20Manager) "SnaggedBarbedWire" (Transformation|GetActorLocation (Variables|Default|GetPlayer))))
    (:CastFailed
      _))
  (bind _asbp_aiinterface (Utilities|Casting|CastToBP_AIInterface OtherActor))
  (Default|SetSpeed _asbp_aiinterface 1.5e+02))

(event OnComponentEndOverlap(BarbedWireFull)
  (params (OverlappedComponent :type Primitive%20Component%20Object%20Reference) (OtherActor :type Actor%20Object%20Reference) (OtherComp :type Primitive%20Component%20Object%20Reference) (OtherBodyIndex :type Integer))
  (bind _asbp_player_movement (Utilities|Casting|CastToBP_PlayerMovement OtherActor)
    (:then
      (Variables|Default|SetPlayerColliding false)
      (Variables|/Script/Engine.CharacterMovementComponent|SetMaxWalkSpeed (Variables|/Script/Engine.Character|GetCharacterMovement _asbp_player_movement) 3e+02)
      (Variables|/Script/ExtractShooter.PlayerMovement|SetStunned _asbp_player_movement false))
    (:CastFailed
      _))
  (bind _asbp_aiinterface (Utilities|Casting|CastToBP_AIInterface OtherActor))
  (Default|SetSpeed _asbp_aiinterface 6e+02))

(event EventBeginPlay)

(event Collision|EventActorBeginOverlap
  (params (OtherActor :type Actor%20Object%20Reference)))

(event EventTick
  (params (DeltaSeconds :type Float%20%28single-precision%29))
  (bind _player (Variables|Default|GetPlayer))
  (if (Variables|Default|GetPlayerColliding)
    (Utilities|FlowControl|Delay 2.0)
    (if (Variables|Default|GetPlayerColliding)
      (Class|PlayerMovement|DealDamagetoPlayer _player 1e+01)
      (Default|PlaySFXbyName (Variables|Default|GetBP%20Audio%20Manager) "SnaggedBarbedWire" (Transformation|GetActorLocation _player)))))

(event EventGetBPAudioManager
  (params (BP%20Audio%20Manager :type BP%20Audio%20Manager%20Object%20Reference))
  (Variables|Default|SetBP%20Audio%20Manager BP%20Audio%20Manager))

(fn ConstructionScript)