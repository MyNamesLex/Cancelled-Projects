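; Cutscene controller that steps through BP_Dialogue lines under black bars, then clears the text or opens the next level, optionally after a music fade.
; BeginPlay resolves two assigned models by cast chains and finds the audio, dialogue and camera actors.
; Each NextDialogue sets the text, snaps the main camera to that line's camera and repositions both models.
; Flags select the robbed or intro cutscene, whose hardcoded Counter branches pick animations.
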(event Custom|NextDialogue
  (bind _bp_dialogue (Variables|Default|GetBP%20Dialogue))
  (bind _nextscenename (Variables|/Script/ExtractShooter.Dialogue|GetNextSceneName _bp_dialogue))
  (if (Utilities|Enum|Equal(Enum) (Utilities|Array|Get(acopy) (Variables|/Script/ExtractShooter.Dialogue|GetDialogue _bp_dialogue) (Variables|Default|GetCounter)) "")
    (if (Variables|/Game/Blueprints/Dialogue/BP_Dialogue.BP_Dialogue_C|GetChangeToSpecificLevelAfterDialogue (Variables|Default|GetBP%20Dialogue))
      (if (Variables|Default|GetFadeOutAudio)
        (Default|FadeOutBGMLoadNextLevel (Variables|Default|GetBP%20Audio%20Manager) 1.0 _nextscenename)
        (else
          (Game|OpenLevel(byName) _nextscenename)))
      (else
        (CallFunction|ExitDialogue)))
    (else
      (bind _output_get (Variables|Default|SetName (Utilities|Array|Get(acopy) (Variables|/Script/ExtractShooter.Dialogue|GetName _bp_dialogue) (Variables|Default|GetCounter))))
      (bind _output_get_2 (Variables|Default|SetDialogue (Utilities|Array|Get(acopy) (Variables|/Script/ExtractShooter.Dialogue|GetDialogue _bp_dialogue) (Variables|Default|GetCounter))))
      (bind _desiredview (Class|CameraComponent|GetCameraView (Variables|/Script/Engine.CameraActor|GetCameraComponent (Utilities|Array|Get(acopy) (Variables|/Script/ExtractShooter.Dialogue|GetCutsceneCamera _bp_dialogue) (Variables|Default|GetCounter))) 5.0))
      (Variables|Default|SetCounter (+ (Variables|Default|GetCounter) 1))
      (if (== (Variables|Default|GetBP%20Dialogue%20Widget) 0) :!label _label
        (Variables|Default|SetBP%20Dialogue%20Widget (Variables|/Game/Blueprints/Dialogue/BP_Dialogue.BP_Dialogue_C|GetBP%20Dialogue%20Widget (Variables|Default|GetBP%20Dialogue)))
        (Utilities|FlowControl|Delay 0.2)
        (goto _label)
        (else
          (Rendering|Components|TextRender|SetText (Variables|/Game/Blueprints/UI/BP_DialogueWidget.BP_DialogueWidget_C|GetNameText (Variables|Default|GetBP%20Dialogue%20Widget)) (Utilities|Text|ToText(String) _output_get))
          (Rendering|Components|TextRender|SetText (Variables|/Game/Blueprints/UI/BP_DialogueWidget.BP_DialogueWidget_C|GetDialogueText (Variables|Default|GetBP%20Dialogue%20Widget)) (Utilities|Text|ToText(String) _output_get_2))
          (Transformation|SetWorldLocationAndRotation (Variables|/Game/Blueprints/Cutscene/BP_PlayerMovementCutscene.BP_PlayerMovementCutscene_C|GetMainCamera (Variables|Default|GetPlayer%20Movement%20Cutscene)) (.location _desiredview) (.rotation _desiredview) false false)
          (CallFunction|GetAnimationtoPlay)
          (Transformation|SetActorLocation (Variables|Default|GetModel1) (Utilities|Array|Get(acopy) (Variables|Default|GetModel1Locations) (Variables|Default|GetCounter)) false false)
          (Transformation|SetActorLocation (Variables|Default|GetModel2) (Utilities|Array|Get(acopy) (Variables|Default|GetModel2Locations) (Variables|Default|GetCounter)) false false)
          (Transformation|SetActorRotation (Variables|Default|GetModel1) (Utilities|Array|Get(acopy) (Variables|Default|GetModel1Rotations) (Variables|Default|GetCounter)))
          (Transformation|SetActorRotation (Variables|Default|GetModel2) (Utilities|Array|Get(acopy) (Variables|Default|GetModel2Rotations) (Variables|Default|GetCounter))))))))

(event Custom|Exit%20Dialogue
  (bind _bp_dialogue_widget (Variables|Default|GetBP%20Dialogue%20Widget))
  (Rendering|Components|TextRender|SetText (Variables|/Game/Blueprints/UI/BP_DialogueWidget.BP_DialogueWidget_C|GetNameText _bp_dialogue_widget) "")
  (Rendering|Components|TextRender|SetText (Variables|/Game/Blueprints/UI/BP_DialogueWidget.BP_DialogueWidget_C|GetDialogueText _bp_dialogue_widget) ""))

(event Custom|GetAnimationToPlay
  (if (Variables|Default|GetPlayerRobbedCutscenee)
    (CallFunction|PlayerRobbedCutscene)
    (elif (Variables|Default|GetIntroCutscene)
      (CallFunction|IntroCutsceneEvent))))

(event Custom|PlayerRobbedCutscene
  (if (== (Variables|Default|GetCounter) 1)
    (Components|Animation|SetAnimation (Variables|/Game/Blueprints/Cutscene/BP_PlayerModelCutscene.BP_PlayerModelCutscene_C|GetPlayer_nonPBR (Variables|Default|GetBP%20Player%20Model)) "/Game/Assets/StillFrames/Player/PlayerHit.PlayerHit")
    (Components|Animation|SetAnimation (Variables|/Game/Blueprints/Cutscene/BP_BossTwoInCutscene.BP_BossTwoInCutscene_C|GetBossTwo (Variables|Default|GetBP%20Boss%20Two)) "/Game/Assets/StillFrames/BossTwo/BossTwoHook.BossTwoHook")
    (elif (== (Variables|Default|GetCounter) 2)
      (Components|Animation|SetAnimation (Variables|/Game/Blueprints/Cutscene/BP_PlayerModelCutscene.BP_PlayerModelCutscene_C|GetPlayer_nonPBR (Variables|Default|GetBP%20Player%20Model)) "/Game/Assets/StillFrames/Player/PlayerOnFloor.PlayerOnFloor")
      (Components|Animation|SetAnimation (Variables|/Game/Blueprints/Cutscene/BP_BossTwoInCutscene.BP_BossTwoInCutscene_C|GetBossTwo (Variables|Default|GetBP%20Boss%20Two)) "/Game/Assets/StillFrames/BossTwo/BossTwoCrouch.BossTwoCrouch")
      (elif (== (Variables|Default|GetCounter) 3)
        (Components|Animation|SetAnimation (Variables|/Game/Blueprints/Cutscene/BP_PlayerModelCutscene.BP_PlayerModelCutscene_C|GetPlayer_nonPBR (Variables|Default|GetBP%20Player%20Model)) "/Game/Assets/StillFrames/Player/PlayerOnFloor.PlayerOnFloor")
        (Components|Animation|SetAnimation (Variables|/Game/Blueprints/Cutscene/BP_BossTwoInCutscene.BP_BossTwoInCutscene_C|GetBossTwo (Variables|Default|GetBP%20Boss%20Two)) "/Game/Assets/StillFrames/BossTwo/BossTwoIdle.BossTwoIdle")
        (elif (== (Variables|Default|GetCounter) 4)
          (Components|Animation|SetAnimation (Variables|/Game/Blueprints/Cutscene/BP_PlayerModelCutscene.BP_PlayerModelCutscene_C|GetPlayer_nonPBR (Variables|Default|GetBP%20Player%20Model)) "/Game/Assets/StillFrames/Player/PlayerOnFloor.PlayerOnFloor")
          (Components|Animation|SetAnimation (Variables|/Game/Blueprints/Cutscene/BP_BossTwoInCutscene.BP_BossTwoInCutscene_C|GetBossTwo (Variables|Default|GetBP%20Boss%20Two)) "/Game/Assets/StillFrames/BossTwo/BossTwoWalk.BossTwoWalk"))))))

(event Custom|IntroCutsceneEvent
  (if (== (Variables|Default|GetCounter) 1)
    (Components|Animation|PlayAnimation (Variables|/Game/Blueprints/Cutscene/BP_BossInCutscene.BP_BossInCutscene_C|GetBossIdle (Variables|Default|GetBP%20Boss)) "/Game/Assets/Models/Boss/BossIdle/BossIdle_Anim.BossIdle_Anim" true)
    (Components|Animation|PlayAnimation (Variables|/Game/Blueprints/Cutscene/BP_BossTwoInCutscene.BP_BossTwoInCutscene_C|GetBossTwo (Variables|Default|GetBP%20Boss%20Two)) "/Game/Assets/Models/Boss/BossIdle/BossIdle_Anim.BossIdle_Anim" true)
    (elif (== (Variables|Default|GetCounter) 2)
      (Components|Animation|PlayAnimation (Variables|/Game/Blueprints/Cutscene/BP_BossInCutscene.BP_BossInCutscene_C|GetBossIdle (Variables|Default|GetBP%20Boss)) "/Game/Assets/Models/Boss/BossIdle/BossIdle_Anim.BossIdle_Anim" true)
      (Components|Animation|PlayAnimation (Variables|/Game/Blueprints/Cutscene/BP_BossTwoInCutscene.BP_BossTwoInCutscene_C|GetBossTwo (Variables|Default|GetBP%20Boss%20Two)) "/Game/Assets/Models/Boss/BossIdle/BossIdle_Anim.BossIdle_Anim" true)
      (elif (== (Variables|Default|GetCounter) 3)
        (Components|Animation|PlayAnimation (Variables|/Game/Blueprints/Cutscene/BP_BossInCutscene.BP_BossInCutscene_C|GetBossIdle (Variables|Default|GetBP%20Boss)) "/Game/Assets/Models/Boss/BossIdle/BossIdle_Anim.BossIdle_Anim" true)
        (Components|Animation|PlayAnimation (Variables|/Game/Blueprints/Cutscene/BP_BossTwoInCutscene.BP_BossTwoInCutscene_C|GetBossTwo (Variables|Default|GetBP%20Boss%20Two)) "/Game/Assets/Models/Boss/BossIdle/BossIdle_Anim.BossIdle_Anim" true)
        (elif (== (Variables|Default|GetCounter) 4)
          (Components|Animation|PlayAnimation (Variables|/Game/Blueprints/Cutscene/BP_BossInCutscene.BP_BossInCutscene_C|GetBossIdle (Variables|Default|GetBP%20Boss)) "/Game/Assets/Models/Boss/BossIdle/BossIdle_Anim.BossIdle_Anim" true)
          (Components|Animation|PlayAnimation (Variables|/Game/Blueprints/Cutscene/BP_BossTwoInCutscene.BP_BossTwoInCutscene_C|GetBossTwo (Variables|Default|GetBP%20Boss%20Two)) "/Game/Assets/Models/Boss/BossIdle/BossIdle_Anim.BossIdle_Anim" true)
          (elif (== (Variables|Default|GetCounter) 5)
            (Components|Animation|PlayAnimation (Variables|/Game/Blueprints/Cutscene/BP_BossInCutscene.BP_BossInCutscene_C|GetBossIdle (Variables|Default|GetBP%20Boss)) "/Game/Assets/Models/Boss/BossIdle/BossIdle_Anim.BossIdle_Anim" true)
            (Components|Animation|PlayAnimation (Variables|/Game/Blueprints/Cutscene/BP_BossTwoInCutscene.BP_BossTwoInCutscene_C|GetBossTwo (Variables|Default|GetBP%20Boss%20Two)) "/Game/Assets/Models/Boss/BossIdle/BossIdle_Anim.BossIdle_Anim" true)))))))

(event EventBeginPlay
  (bind _model2 (Variables|Default|GetModel2))
  (bind _model1 (Variables|Default|GetModel1))
  (bind _returnvalue (Actor|GetActorOfClass "/Game/Blueprints/Audio/BP_AudioManager.BP_AudioManager_C"))
  (Variables|Default|SetBP%20Audio%20Manager _returnvalue)
  (bind _asbp_boss_in_cutscene (Utilities|Casting|CastToBP_BossInCutscene _model1)
    (:then
      (Variables|Default|SetBP%20Boss _asbp_boss_in_cutscene))
    (:CastFailed
      (bind _asbp_boss_two_in_cutscene (Utilities|Casting|CastToBP_BossTwoInCutscene _model1)
        (:then
          (Variables|Default|SetBP%20Boss%20Two _asbp_boss_two_in_cutscene))
        (:CastFailed
          (bind _asbp_player_model_cutscene (Utilities|Casting|CastToBP_PlayerModelCutscene _model1)
            (:then
              (Variables|Default|SetBP%20Player%20Model _asbp_player_model_cutscene))
            (:CastFailed
              (Development|PrintString "BP CUTSCENE CONTROL MODEL 1 NOT FOUND")))))))
  (bind _asbp_boss_in_cutscene_2 (Utilities|Casting|CastToBP_BossInCutscene _model2)
    (:then
      (Variables|Default|SetBP%20Boss _asbp_boss_in_cutscene_2))
    (:CastFailed
      (bind _asbp_boss_two_in_cutscene_2 (Utilities|Casting|CastToBP_BossTwoInCutscene _model2)
        (:then
          (Variables|Default|SetBP%20Boss%20Two _asbp_boss_two_in_cutscene_2))
        (:CastFailed
          (bind _asbp_player_model_cutscene_2 (Utilities|Casting|CastToBP_PlayerModelCutscene _model2)
            (:then
              (Variables|Default|SetBP%20Player%20Model _asbp_player_model_cutscene_2))
            (:CastFailed
              (Development|PrintString "BP CUTSCENE CONTROL MODEL 2 NOT FOUND")))))))
  (bind _returnvalue_2 (Actor|GetActorOfClass "/Game/Blueprints/Cutscene/BP_PlayerMovementCutscene.BP_PlayerMovementCutscene_C"))
  (Variables|Default|SetPlayer%20Movement%20Cutscene _returnvalue_2)
  (bind _returnvalue_3 (Actor|GetActorOfClass "/Game/Blueprints/Dialogue/BP_Dialogue.BP_Dialogue_C"))
  (bind _output_get (Variables|Default|SetBP%20Dialogue _returnvalue_3))
  (if (Variables|/Game/Blueprints/Dialogue/BP_Dialogue.BP_Dialogue_C|GetOnBeginPlay _output_get)
    (Variables|Default|SetBP%20Dialogue%20Widget (Variables|/Game/Blueprints/Dialogue/BP_Dialogue.BP_Dialogue_C|GetBP%20Dialogue%20Widget (Variables|Default|GetBP%20Dialogue)))
    (CallFunction|NextDialogue)
    (bind _returnvalue_4 (UserInterface|CreateWidget "/Game/Blueprints/UI/BP_UIBlackBars.BP_UIBlackBars_C"))
    (UserInterface|Viewport|AddtoViewport _returnvalue_4 -99)))

(event Collision|EventActorBeginOverlap
  (params (OtherActor :type Actor%20Object%20Reference)))

(event EventTick
  (params (DeltaSeconds :type Float%20%28single-precision%29)))

(fn ConstructionScript)