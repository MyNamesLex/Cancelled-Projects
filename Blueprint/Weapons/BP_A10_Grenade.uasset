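; A10 grenade weapon that is a pickup item and, once thrown, explodes to damage and stun AI and players.
; Pickup returns its item stats and teleports the actor below the world.
; A hit while Thrown calls Explode, which enables Sphere overlaps, spawns effects, plays audio through BP_AudioManager, then destroys the actor after a short delay.
; Sphere overlaps apply damage and stun, then re-call Explode on itself via BP_ExplosionInterface.
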(event OnComponentBeginOverlap(Sphere)
  (params (OverlappedComponent :type Primitive%20Component%20Object%20Reference) (OtherActor :type Actor%20Object%20Reference) (OtherComp :type Primitive%20Component%20Object%20Reference) (OtherBodyIndex :type Integer) (bFromSweep :type Boolean) (SweepResult :type Hit%20Result%20Structure%20%28by%20ref%29))
  (bind _damage (Variables|Default|GetDamage))
  (bind _asbp_aiinterface (Utilities|Casting|CastToBP_AIInterface OtherActor)
    (:then
      (Default|DamageDeal _asbp_aiinterface _damage)
      (Default|Stunned _asbp_aiinterface))
    (:CastFailed
      _))
  (bind _asbp_player_movement (Utilities|Casting|CastToBP_PlayerMovement OtherActor)
    (:then
      (Class|PlayerMovement|DealDamagetoPlayer _asbp_player_movement (Math|Conversions|ToFloat(Integer) _damage))
      (Default|StunnedFunc _asbp_player_movement))
    (:CastFailed
      _))
  (if (== OtherComp 0)
    _
    (else
      _))
  (bind _asbp_explosion_interface (Utilities|Casting|CastToBP_ExplosionInterface self))
  (Default|Explode _asbp_explosion_interface))

(event OnComponentHit(A10_Grenade)
  (params (HitComponent :type Primitive%20Component%20Object%20Reference) (OtherActor :type Actor%20Object%20Reference) (OtherComp :type Primitive%20Component%20Object%20Reference) (NormalImpulse :type Vector :default "0, 0, 0") (Hit :type Hit%20Result%20Structure%20%28by%20ref%29))
  (if (Variables|Default|GetThrown)
    (CallFunction|Explode)))

(event Custom|DestroyItem
  (Utilities|FlowControl|Delay 0.1)
  (Transformation|SetActorLocation "0, 0,-999.000000" false true))

(event EventExplode
  (bind _a10_grenade (Variables|Default|GetA10_Grenade))
  (bind _returnvalue (Transformation|GetWorldLocation _a10_grenade))
  (Variables|/Script/Engine.PrimitiveComponent|SetbGenerateOverlapEvents (Variables|Default|GetSphere) true)
  (Niagara|SpawnSystematLocation "/Game/Assets/Niagara/Traps/Outer_Mine_Explosion.Outer_Mine_Explosion" _returnvalue "0, 0, 0" "2.000000,2.000000,2.000000")
  (Default|PlaySFXbyName (Variables|Default|GetBP%20Audio%20Manager) "Explosion" _returnvalue)
  (Utilities|FlowControl|Delay 0.2)
  (Actor|DestroyActor))

(event Collision|EventActorBeginOverlap
  (params (OtherActor :type Actor%20Object%20Reference)))

(event EventTick
  (params (DeltaSeconds :type Float%20%28single-precision%29))
  (Rendering|SetVisibility (Variables|Default|GetSphere) false false))

(event EventBeginPlay
  (bind _returnvalue (Actor|GetActorOfClass "/Game/Blueprints/Audio/BP_AudioManager.BP_AudioManager_C"))
  (Variables|Default|SetBP%20Audio%20Manager _returnvalue))

(event Collision|EventHit
  (params (MyComp :type Primitive%20Component%20Object%20Reference) (Other :type Actor%20Object%20Reference) (OtherComp :type Primitive%20Component%20Object%20Reference) (bSelfMoved :type Boolean) (HitLocation :type Vector :default "0, 0, 0") (HitNormal :type Vector :default "0, 0, 0") (NormalImpulse :type Vector :default "0, 0, 0") (Hit :type Hit%20Result%20Structure%20%28by%20ref%29))
  (if (Variables|Default|GetThrown)
    (CallFunction|Explode)))

(fn ConstructionScript)

(fn PickUpItem
  (Development|PrintString "Item Picked Up")
  (CallFunction|DestroyItem)
  (return (Variables|Default|GetItem) (Variables|Default|GetWeaponType) (Variables|Default|GetDamage) (Variables|Default|GetWeaponRecoil) (Variables|Default|GetMagSize) (Variables|Default|GetFireRate) (Variables|Default|GetA10_Grenade) (Variables|Default|GetItemType) "" "" "" "" false 0 0 0 0))

(fn SetItemStats
  (params (Damage :type Integer) (WeaponType :type String) (ItemName :type String) (WeaponRecoil :type Float%20%28double-precision%29) (MagSize :type Integer) (FireRate :type Float%20%28double-precision%29) (ItemType :type String) (SpeedBoostDuration :type String) (SpeedBoostIntensity :type String) (HealIntensity :type String) (HealDuration :type String) (CanADS :type Boolean) (Rifle%20Ammo :type Integer) (Sniper%20Ammo :type Integer) (Shotgun%20Ammo :type Integer) (Pistol%20Ammo :type Integer))
  (Variables|Default|SetDamage Damage)
  (Variables|Default|SetItem ItemName)
  (Variables|Default|SetWeaponType WeaponType)
  (Variables|Default|SetWeaponRecoil WeaponRecoil)
  (Variables|Default|SetMagSize MagSize)
  (Variables|Default|SetFireRate FireRate)
  (Variables|Default|SetItemType ItemType)
  (return))