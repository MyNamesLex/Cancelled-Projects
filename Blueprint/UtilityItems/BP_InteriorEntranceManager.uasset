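; BP_InteriorEntranceManager keeps killed enemies and picked-up items gone when interior and outdoor maps reload, storing state in the GameInstance.
; It tags enemies and items by array index, retrying until found and triggering RNG item spawning if needed.
; Deaths save to per-level arrays chosen by level name; items at Z -999 count as picked up.
; When InLevel is already set, BeginPlay destroys the recorded actors by tag.
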(event Custom|SetRemovePickedUpItems
  (Development|PrintString "SetRemovePickedUpItems")
  (for _array_element (Variables|/Game/Blueprints/BP_GameInstance.BP_GameInstance_C|GetItems (Variables|Default|GetGame%20Instance))
    (bind _outactors (Actor|GetAllActorswithTag _array_element))
    (if (not (== (Utilities|Array|Get(acopy) _outactors) 0))
      (if (== (.z (Transformation|GetActorLocation (Utilities|Array|Get(acopy) _outactors))) -999.0)
        (Utilities|Array|Add (Variables|/Game/Blueprints/BP_GameInstance.BP_GameInstance_C|GetPickedUpItems (Variables|Default|GetGame%20Instance)) _array_element)))))

(event Custom|SetItemTags
  (Utilities|FlowControl|Delay 1.0)
  (Development|PrintString "SetItemTags")
  (bind _outactors (Actor|GetAllActorswithInterface "/Game/Blueprints/Inventory/BP_ItemStats.BP_ItemStats_C" :!label _label))
  (if (<= (Utilities|Array|Length _outactors) 1)
    (Utilities|FlowControl|Delay 0.2)
    (Development|PrintString "NO ITEMS FOUND, RETRYING ")
    (bind _returnvalue (Actor|GetActorOfClass "/Game/Blueprints/UtilityItems/BP_RNGItemSpawn.BP_RNGItemSpawn_C"))
    (if (not (== _returnvalue 0))
      (Default|StartRNGItemSpawn _returnvalue)
      (Utilities|FlowControl|Delay 1.0)
      (goto _label))
    (else
      (for (_array_element _array_index) _outactors
        (Variables|/Script/Engine.Actor|SetTags _array_element (Utilities|Array|MakeArray (Utilities|Array|Get(acopy) (Variables|Default|GetItemsTagsArray) _array_index)))
        (Utilities|Array|Add (Variables|/Game/Blueprints/BP_GameInstance.BP_GameInstance_C|GetItems (Variables|Default|GetGame%20Instance)) (Utilities|Array|Get(acopy) (Variables|Default|GetItemsTagsArray) _array_index))
        (Development|PrintString "set item tag ")
        (Development|PrintString (Utilities|String|ToString(Integer) _array_index)))
      (Development|PrintString "SET ALL ITEM TAGS"))))

(event Custom|SetEnemyTags
  (bind _game_instance (Variables|Default|GetGame%20Instance))
  (bind _enemies (Variables|/Game/Blueprints/BP_GameInstance.BP_GameInstance_C|GetEnemies _game_instance))
  (Development|PrintString "SET ENEMY TAG")
  (bind _outactors (Actor|GetAllActorswithInterface "/Game/Blueprints/AI/BP_AIInterface.BP_AIInterface_C" :!label _label))
  (if (<= (Utilities|Array|Length _outactors) 1)
    (Development|PrintString "cant find bp ai interface bp interiorentrancemanager")
    (Utilities|FlowControl|Delay 0.2)
    (goto _label)
    (else
      (for (_array_element _array_index) _outactors
        (Variables|/Script/Engine.Actor|SetTags _array_element (Utilities|Array|MakeArray (Utilities|Array|Get(acopy) (Variables|Default|GetEnemiesTagsArray) _array_index)))
        (if (not (Utilities|Array|ContainsItem _enemies (Utilities|String|StringToName (Utilities|String|ToString(Integer) _array_index))))
          (Utilities|Array|Add _enemies (Utilities|String|StringToName (Utilities|String|ToString(Integer) _array_index))))))))

(event Custom|SetDeadEnemiesFunc
  (params (tag :type Name))
  (Development|PrintString "SET DEAD ENEMIES FUNC")
  (bind _outactors (Actor|GetAllActorswithTag tag))
  (bind _health (Class|BPAIInterface|GetHealth(Message) (Utilities|Array|Get(acopy) _outactors)))
  (if (<= _health 0.0)
    (bind _deadenemies (CallFunction|GetDeadEnemies))
    (if (not (Utilities|Array|ContainsItem _deadenemies tag))
      (Utilities|Array|Add _deadenemies tag)
      (Development|PrintString (Utilities|String|ToString(Name) tag) true true "(R=0.000000,G=1.000000,B=0.143308,A=1.000000)")
      (Development|PrintString "DEAD ENEMY ADDED")
      (CallFunction|SetDeadEnemies _deadenemies))))

(event Custom|RemoveAllPickedUpItems
  (Development|PrintString "RemoveAllPickedUpItems")
  (Utilities|Array|Clear (Variables|/Game/Blueprints/BP_GameInstance.BP_GameInstance_C|GetItems (Variables|Default|GetGame%20Instance)))
  (CallFunction|SetItemTags)
  (Utilities|FlowControl|Delay 1.0)
  (for _array_element (Variables|/Game/Blueprints/BP_GameInstance.BP_GameInstance_C|GetPickedUpItems (Variables|Default|GetGame%20Instance))
    (bind _outactors (Actor|GetAllActorswithTag _array_element))
    (if (!= (Utilities|Array|Get(acopy) _outactors) 0)
      (Actor|DestroyActor (Utilities|Array|Get(acopy) _outactors))
      (Development|PrintString "Destroyed item Picked Up"))))

(event Custom|KillDeadEnemies
  (CallFunction|SetEnemyTags)
  (Development|PrintString "KILLDEADENEMIES")
  (Utilities|FlowControl|Delay 0.2)
  (bind _deadenemies (CallFunction|GetDeadEnemies))
  (Utilities|FlowControl|Delay 0.2)
  (Development|PrintString (Utilities|String|ToString(Integer) (Utilities|Array|Length _deadenemies)))
  (Development|PrintString "DEAD ENEMIES LENGTH MESSAGE PRIOR")
  (for _array_element _deadenemies
    (bind _outactors (Actor|GetAllActorswithTag _array_element))
    (if (not (== (Utilities|Array|Get(acopy) _outactors) 0))
      (Actor|DestroyActor (Utilities|Array|Get(acopy) _outactors))
      (Development|PrintString "KILLED AN AI")
      (Development|PrintString (Utilities|GetDisplayName (Utilities|Array|Get(acopy) _outactors))))))

(event EventBeginPlay
  (bind _asbp_game_instance (Utilities|Casting|CastToBP_GameInstance (Game|GetGameInstance)))
  (bind _output_get (Variables|Default|SetGame%20Instance _asbp_game_instance))
  (Variables|/Game/Blueprints/BP_GameInstance.BP_GameInstance_C|SetEnemies _output_get (Variables|Default|GetNULLNAMEARRAY))
  (if (Variables|/Game/Blueprints/BP_GameInstance.BP_GameInstance_C|GetInLevel _output_get)
    (CallFunction|SetEnemyTags)
    (CallFunction|SetItemTags)
    (Utilities|FlowControl|Delay 3.0)
    (CallFunction|KillDeadEnemies)
    (CallFunction|RemoveAllPickedUpItems)
    (else
      (Variables|/Game/Blueprints/BP_GameInstance.BP_GameInstance_C|SetInLevel (Variables|Default|GetGame%20Instance) true)
      (CallFunction|SetEnemyTags)
      (CallFunction|SetItemTags))))

(event Collision|EventActorBeginOverlap
  (params (OtherActor :type Actor%20Object%20Reference)))

(event EventTick
  (params (DeltaSeconds :type Float%20%28single-precision%29)))

(fn ConstructionScript)

(fn GetDeadEnemies
  (bind _game_instance (Variables|Default|GetGame%20Instance))
  (bind _returnvalue (Game|GetCurrentLevelName true))
  (switch string _returnvalue
    (:Default
      (Development|PrintString "GET DEAD ENEMIES DEFAULT HIT"))
    (:TutorialMapLevel6House1Interior
      (LocalVariables|SetDead%20Enemies (Variables|/Game/Blueprints/BP_GameInstance.BP_GameInstance_C|GetInteriorDeadEnemiesTutorialMapLevel6House1Interior _game_instance))
      (return (LocalVariables|GetDead%20Enemies)))
    (:TutorialMapLevel6House2Interior
      (LocalVariables|SetDead%20Enemies (Variables|/Game/Blueprints/BP_GameInstance.BP_GameInstance_C|GetInteriorDeadEnemiesTutorialMapLevel6House2Interior _game_instance))
      (return (LocalVariables|GetDead%20Enemies)))
    (:NormalMapLevel1House1Interior
      (LocalVariables|SetDead%20Enemies (Variables|/Game/Blueprints/BP_GameInstance.BP_GameInstance_C|GetInteriorDeadEnemiesNormalMapLevel1House1Interior _game_instance))
      (return (LocalVariables|GetDead%20Enemies)))
    (:NormalMapLevel1House2Interior
      (LocalVariables|SetDead%20Enemies (Variables|/Game/Blueprints/BP_GameInstance.BP_GameInstance_C|GetInteriorDeadEnemiesNormalMapLevel1House2Interior _game_instance))
      (return (LocalVariables|GetDead%20Enemies)))
    (:NormalMapLevel2OfficeInterior
      (LocalVariables|SetDead%20Enemies (Variables|/Game/Blueprints/BP_GameInstance.BP_GameInstance_C|GetInteriorDeadEnemiesNormalMapLevel2OfficeInterior _game_instance))
      (return (LocalVariables|GetDead%20Enemies)))
    (:NormalMapLevel3ShopInterior
      (LocalVariables|SetDead%20Enemies (Variables|/Game/Blueprints/BP_GameInstance.BP_GameInstance_C|GetInteriorDeadEnemiesNormalMapLevel3ShopInterior _game_instance))
      (return (LocalVariables|GetDead%20Enemies)))
    (:NormalMapLevel5GunStoreInterior
      (LocalVariables|SetDead%20Enemies (Variables|/Game/Blueprints/BP_GameInstance.BP_GameInstance_C|GetInteriorDeadEnemiesNormalMapLevel5GunStoreInterior _game_instance))
      (return (LocalVariables|GetDead%20Enemies)))
    (:NormalMapLevel5House1Interior
      (LocalVariables|SetDead%20Enemies (Variables|/Game/Blueprints/BP_GameInstance.BP_GameInstance_C|GetInteriorDeadEnemiesNormalMapLevel5House1Interior _game_instance))
      (return (LocalVariables|GetDead%20Enemies)))
    (:NormalMapLevel5House2Interior
      (LocalVariables|SetDead%20Enemies (Variables|/Game/Blueprints/BP_GameInstance.BP_GameInstance_C|GetInteriorDeadEnemiesNormalMapLevel5House2Interior _game_instance))
      (return (LocalVariables|GetDead%20Enemies)))
    (:NormalMapLevel5House3Interior
      (LocalVariables|SetDead%20Enemies (Variables|/Game/Blueprints/BP_GameInstance.BP_GameInstance_C|GetInteriorDeadEnemiesNormalMapLevel5House3Interior _game_instance))
      (return (LocalVariables|GetDead%20Enemies)))
    (:NormalMapLevel5House4Interior
      (LocalVariables|SetDead%20Enemies (Variables|/Game/Blueprints/BP_GameInstance.BP_GameInstance_C|GetInteriorDeadEnemiesNormalMapLevel5House4Interior _game_instance))
      (return (LocalVariables|GetDead%20Enemies)))
    (:NormalMapLevel5House5Interior
      (LocalVariables|SetDead%20Enemies (Variables|/Game/Blueprints/BP_GameInstance.BP_GameInstance_C|GetInteriorDeadEnemiesNormalMapLevel5House5Interior _game_instance))
      (return (LocalVariables|GetDead%20Enemies)))
    (:NormalMapLevel5House6Interior
      (LocalVariables|SetDead%20Enemies (Variables|/Game/Blueprints/BP_GameInstance.BP_GameInstance_C|GetInteriorDeadEnemiesNormalMapLevel5House6Interior _game_instance))
      (return (LocalVariables|GetDead%20Enemies)))
    (:NormalMapLevel5House7Interior
      (LocalVariables|SetDead%20Enemies (Variables|/Game/Blueprints/BP_GameInstance.BP_GameInstance_C|GetInteriorDeadEnemiesNormalMapLevel5House7Interior _game_instance))
      (return (LocalVariables|GetDead%20Enemies)))
    (:NormalMapLevel6FarmhouseInterior
      (LocalVariables|SetDead%20Enemies (Variables|/Game/Blueprints/BP_GameInstance.BP_GameInstance_C|GetInteriorDeadEnemiesNormalMapLevel6FarmhouseInterior _game_instance))
      (return (LocalVariables|GetDead%20Enemies)))
    (:NormalMapLevel1
      (LocalVariables|SetDead%20Enemies (Variables|/Game/Blueprints/BP_GameInstance.BP_GameInstance_C|GetDeadEnemiesNormalMapLevel1 _game_instance))
      (return (LocalVariables|GetDead%20Enemies)))
    (:NormalMapLevel2
      (LocalVariables|SetDead%20Enemies (Variables|/Game/Blueprints/BP_GameInstance.BP_GameInstance_C|GetDeadEnemiesNormalMapLevel2 _game_instance))
      (return (LocalVariables|GetDead%20Enemies)))
    (:NormalMapLevel3
      (Development|PrintString "NormalMapLevel3 Found Get Dead Enemies")
      (LocalVariables|SetDead%20Enemies (Variables|/Game/Blueprints/BP_GameInstance.BP_GameInstance_C|GetDeadEnemiesNormalMapLevel3 _game_instance))
      (return (LocalVariables|GetDead%20Enemies)))
    (:NormalMapLevel4
      (LocalVariables|SetDead%20Enemies (Variables|/Game/Blueprints/BP_GameInstance.BP_GameInstance_C|GetDeadEnemiesNormalMapLevel4 _game_instance))
      (return (LocalVariables|GetDead%20Enemies)))
    (:NormalMapLevel5
      (LocalVariables|SetDead%20Enemies (Variables|/Game/Blueprints/BP_GameInstance.BP_GameInstance_C|GetDeadEnemiesNormalMapLevel5 _game_instance))
      (return (LocalVariables|GetDead%20Enemies)))
    (:NormalMapLevel6
      (LocalVariables|SetDead%20Enemies (Variables|/Game/Blueprints/BP_GameInstance.BP_GameInstance_C|GetDeadEnemiesNormalMapLevel6 _game_instance))
      (return (LocalVariables|GetDead%20Enemies)))
    (:TutorialMapLevel6
      (LocalVariables|SetDead%20Enemies (Variables|/Game/Blueprints/BP_GameInstance.BP_GameInstance_C|GetDeadEnemiesTutorialMapLevel6 _game_instance))
      (return (LocalVariables|GetDead%20Enemies)))
    (:NormalMapLevel6FarmhouseInteriorNew
      (LocalVariables|SetDead%20Enemies (Variables|/Game/Blueprints/BP_GameInstance.BP_GameInstance_C|GetInteriorDeadEnemiesNormalMapLevel6FarmhouseInteriorNew _game_instance))
      (return (LocalVariables|GetDead%20Enemies)))))

(fn SetDeadEnemies
  (params (Dead%20Enemies :type Array%20of%20Names))
  (bind _game_instance (Variables|Default|GetGame%20Instance))
  (bind _returnvalue (Game|GetCurrentLevelName true))
  (switch string _returnvalue
    (:TutorialMapLevel6House1Interior
      (Variables|/Game/Blueprints/BP_GameInstance.BP_GameInstance_C|SetInteriorDeadEnemiesTutorialMapLevel6House1Interior _game_instance Dead%20Enemies))
    (:TutorialMapLevel6House2Interior
      (Variables|/Game/Blueprints/BP_GameInstance.BP_GameInstance_C|SetInteriorDeadEnemiesNormalMapLevel1House2Interior _game_instance Dead%20Enemies))
    (:NormalMapLevel1House1Interior
      (Variables|/Game/Blueprints/BP_GameInstance.BP_GameInstance_C|SetInteriorDeadEnemiesNormalMapLevel1House1Interior _game_instance Dead%20Enemies))
    (:NormalMapLevel1House2Interior
      (Variables|/Game/Blueprints/BP_GameInstance.BP_GameInstance_C|SetInteriorDeadEnemiesNormalMapLevel1House2Interior _game_instance Dead%20Enemies))
    (:NormalMapLevel2OfficeInterior
      (Variables|/Game/Blueprints/BP_GameInstance.BP_GameInstance_C|SetInteriorDeadEnemiesNormalMapLevel2OfficeInterior _game_instance Dead%20Enemies))
    (:NormalMapLevel3ShopInterior
      (Variables|/Game/Blueprints/BP_GameInstance.BP_GameInstance_C|SetInteriorDeadEnemiesNormalMapLevel3ShopInterior _game_instance Dead%20Enemies))
    (:NormalMapLevel5GunStoreInterior
      (Variables|/Game/Blueprints/BP_GameInstance.BP_GameInstance_C|SetInteriorDeadEnemiesNormalMapLevel5GunStoreInterior _game_instance Dead%20Enemies))
    (:NormalMapLevel5House1Interior
      (Variables|/Game/Blueprints/BP_GameInstance.BP_GameInstance_C|SetInteriorDeadEnemiesNormalMapLevel5House1Interior _game_instance Dead%20Enemies))
    (:NormalMapLevel5House2Interior
      (Variables|/Game/Blueprints/BP_GameInstance.BP_GameInstance_C|SetInteriorDeadEnemiesNormalMapLevel5House2Interior _game_instance Dead%20Enemies))
    (:NormalMapLevel5House3Interior
      (Variables|/Game/Blueprints/BP_GameInstance.BP_GameInstance_C|SetInteriorDeadEnemiesNormalMapLevel5House3Interior _game_instance Dead%20Enemies))
    (:NormalMapLevel5House4Interior
      (Variables|/Game/Blueprints/BP_GameInstance.BP_GameInstance_C|SetInteriorDeadEnemiesNormalMapLevel5House4Interior _game_instance Dead%20Enemies))
    (:NormalMapLevel5House5Interior
      (Variables|/Game/Blueprints/BP_GameInstance.BP_GameInstance_C|SetInteriorDeadEnemiesNormalMapLevel5House5Interior _game_instance Dead%20Enemies))
    (:NormalMapLevel5House6Interior
      (Variables|/Game/Blueprints/BP_GameInstance.BP_GameInstance_C|SetInteriorDeadEnemiesNormalMapLevel5House6Interior _game_instance Dead%20Enemies))
    (:NormalMapLevel5House7Interior
      (Variables|/Game/Blueprints/BP_GameInstance.BP_GameInstance_C|SetInteriorDeadEnemiesNormalMapLevel5House7Interior _game_instance Dead%20Enemies))
    (:NormalMapLevel6FarmhouseInterior
      (Variables|/Game/Blueprints/BP_GameInstance.BP_GameInstance_C|SetInteriorDeadEnemiesNormalMapLevel6FarmhouseInterior _game_instance Dead%20Enemies))
    (:NormalMapLevel1
      (Variables|/Game/Blueprints/BP_GameInstance.BP_GameInstance_C|SetDeadEnemiesNormalMapLevel1 _game_instance Dead%20Enemies))
    (:NormalMapLevel2
      (Variables|/Game/Blueprints/BP_GameInstance.BP_GameInstance_C|SetDeadEnemiesNormalMapLevel2 _game_instance Dead%20Enemies))
    (:NormalMapLevel3
      (Variables|/Game/Blueprints/BP_GameInstance.BP_GameInstance_C|SetDeadEnemiesNormalMapLevel3 _game_instance Dead%20Enemies))
    (:NormalMapLevel4
      (Variables|/Game/Blueprints/BP_GameInstance.BP_GameInstance_C|SetDeadEnemiesNormalMapLevel4 _game_instance Dead%20Enemies))
    (:NormalMapLevel5
      (Variables|/Game/Blueprints/BP_GameInstance.BP_GameInstance_C|SetDeadEnemiesNormalMapLevel5 _game_instance Dead%20Enemies))
    (:NormalMapLevel6
      (Variables|/Game/Blueprints/BP_GameInstance.BP_GameInstance_C|SetDeadEnemiesNormalMapLevel6 _game_instance Dead%20Enemies))
    (:TutorialMapLevel6
      (Variables|/Game/Blueprints/BP_GameInstance.BP_GameInstance_C|SetDeadEnemiesTutorialMapLevel6 _game_instance Dead%20Enemies))
    (:NormalMapLevel6FarmhouseeInteriorNew
      (Variables|/Game/Blueprints/BP_GameInstance.BP_GameInstance_C|SetInteriorDeadEnemiesNormalMapLevel6FarmhouseInteriorNew _game_instance Dead%20Enemies))))