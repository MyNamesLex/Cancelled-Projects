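; Utility actor that watches a referenced boss AI for death and can trigger a follow-up dialogue.
; Each Tick it polls the AI's health through BP_AIInterface, with a one-shot Lock so death or a missing interface is handled only once.
; On death, if enabled, it flags the player as in dialogue, waits briefly, then calls NextDialogueNoCutscene on the assigned dialogue.
; BeginPlay caches the level name, which goes unused here.
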(event EventBeginPlay
  (bind _returnvalue (Game|GetCurrentLevelName true))
  (Variables|Default|SetLevelName (Utilities|String|StringToName _returnvalue)))

(event Collision|EventActorBeginOverlap
  (params (OtherActor :type Actor%20Object%20Reference)))

(event EventTick
  (params (DeltaSeconds :type Float%20%28single-precision%29))
  (bind _aitocheck (Variables|Default|GetAIToCheck))
  (if (Utilities|DoesObjectImplementInterface _aitocheck "/Game/Blueprints/AI/BP_AIInterface.BP_AIInterface_C")
    (bind _health (Class|BPAIInterface|GetHealth(Message) _aitocheck))
    (if (<= _health 0.0)
      (if (not (Variables|Default|GetLock))
        (Variables|Default|SetLock true)
        (Development|PrintString "AITOCHECK IS DEAD BP CHECK FOR DEAD BOSS")
        (if (Variables|Default|GetDialogueAfterDeadAI?)
          (bind _returnvalue (Actor|GetActorOfClass "/Game/Blueprints/Player/BP_PlayerMovement.BP_PlayerMovement_C"))
          (Variables|/Script/ExtractShooter.PlayerMovement|SetisInDialogue _returnvalue true)
          (Utilities|FlowControl|Delay 1.0)
          (Default|NextDialogueNoCutscene (Variables|Default|GetDialogueToPlayAfterDialogue)))))
    (elif (not (Variables|Default|GetLock))
      (Variables|Default|SetLock true)
      (Development|PrintString "AITOCHECK DOES NOT IMPLEMENT BP_AIINTERFACE BP CHECK FOR DEAD BOSS "))))

(fn ConstructionScript)