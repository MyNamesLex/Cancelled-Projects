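; BP_BlockExitTutMapLevel1-1 is a blocker on the tutorial map exit that holds the player back until tutorial progress is far enough.
; When the player hits its cube, it destroys itself if the BP_PopupTypewriterText counter has reached WhenToAllowExit.
; Otherwise it shows a player UI hint naming whichever of the speed and health packs is unused, based on two flags this graph only reads.
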(event OnComponentHit(Cube)
  (params (HitComponent :type Primitive%20Component%20Object%20Reference) (OtherActor :type Actor%20Object%20Reference) (OtherComp :type Primitive%20Component%20Object%20Reference) (NormalImpulse :type Vector :default "0, 0, 0") (Hit :type Hit%20Result%20Structure%20%28by%20ref%29))
  (bind _asbp_player_movement (Utilities|Casting|CastToBP_PlayerMovement OtherActor))
  (bind _returnvalue (Actor|GetActorOfClass "/Game/Blueprints/UI/BP_PopupTypewriterText.BP_PopupTypewriterText_C"))
  (bind _asbp_popup_typewriter_text (Utilities|Casting|CastToBP_PopupTypewriterText _returnvalue))
  (if (>= (Variables|/Game/Blueprints/UI/BP_PopupTypewriterText.BP_PopupTypewriterText_C|GetCounter _asbp_popup_typewriter_text) (Variables|Default|GetWhen%20To%20Allow%20Exit))
    (Actor|DestroyActor)
    (else
      (CallFunction|ShowPopup))))

(event Custom|ShowPopup
  (if (and (== (Variables|Default|GetUsedSpeedPack) false) (Variables|Default|GetUsedHealthPack))
    (Class|PlayerMovement|CallPlayerUIPopupText (stale OnComponentHit(Cube) _asbp_player_movement) "I Need To Use The Speed Pack" 5.0)
    (elif (and (== (Variables|Default|GetUsedHealthPack) false) (Variables|Default|GetUsedSpeedPack))
      (Class|PlayerMovement|CallPlayerUIPopupText (stale OnComponentHit(Cube) _asbp_player_movement) "I Need To Use The Health Pack..." 5.0)
      (elif (and (== (Variables|Default|GetUsedHealthPack) false) (== (Variables|Default|GetUsedSpeedPack) false))
        (Class|PlayerMovement|CallPlayerUIPopupText (stale OnComponentHit(Cube) _asbp_player_movement) "I Need To Use The Speed Pack And Health Pack..." 5.0)))))

(event EventBeginPlay)

(event Collision|EventActorBeginOverlap
  (params (OtherActor :type Actor%20Object%20Reference)))

(event EventTick
  (params (DeltaSeconds :type Float%20%28single-precision%29)))

(fn ConstructionScript)