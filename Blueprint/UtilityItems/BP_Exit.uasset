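; Level exit trigger that lets the regular or tutorial player leave the current level.
; Cube overlap shows a "Leave Level?" popup, and Tick polls the player's LeaveLevel flag while overlapping.
; Exit clears game instance level data, saves regular player stats, locks and optionally waits for music fade-out.
; Tutorial levels then open LevelToOpen, while others open a random BP_LevelTracker level, retrying on None.
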(event OnComponentBeginOverlap(Cube)
  (params (OverlappedComponent :type Primitive%20Component%20Object%20Reference) (OtherActor :type Actor%20Object%20Reference) (OtherComp :type Primitive%20Component%20Object%20Reference) (OtherBodyIndex :type Integer) (bFromSweep :type Boolean) (SweepResult :type Hit%20Result%20Structure%20%28by%20ref%29))
  (bind _asbp_player_movement (Utilities|Casting|CastToBP_PlayerMovement OtherActor)
    (:then
      (Variables|/Script/ExtractShooter.PlayerMovement|SetOverlappingLevelEnterOrExit _asbp_player_movement true)
      (Variables|Default|Setoverlapping true)
      (Class|PlayerMovement|CallPlayerUIPopupText _asbp_player_movement "Leave Level? \"L\"" 1e+69))
    (:CastFailed
      (bind _asbp_player_movement_tutorial (Utilities|Casting|CastToBP_PlayerMovementTutorial OtherActor))
      (Variables|/Script/ExtractShooter.PlayerMovement|SetOverlappingLevelEnterOrExit _asbp_player_movement_tutorial true)
      (Variables|Default|Setoverlapping true)
      (Class|PlayerMovement|CallPlayerUIPopupText _asbp_player_movement_tutorial "Leave Level? \"L\"" 1e+69))))

(event OnComponentEndOverlap(Cube)
  (params (OverlappedComponent :type Primitive%20Component%20Object%20Reference) (OtherActor :type Actor%20Object%20Reference) (OtherComp :type Primitive%20Component%20Object%20Reference) (OtherBodyIndex :type Integer))
  (bind _asbp_player_movement (Utilities|Casting|CastToBP_PlayerMovement OtherActor)
    (:then
      (Variables|/Script/ExtractShooter.PlayerMovement|SetOverlappingLevelEnterOrExit _asbp_player_movement false)
      (Variables|Default|Setoverlapping false)
      (Class|PlayerMovement|CallRemovePlayerUIPopupText _asbp_player_movement))
    (:CastFailed
      (bind _asbp_player_movement_tutorial (Utilities|Casting|CastToBP_PlayerMovementTutorial OtherActor))
      (Variables|/Script/ExtractShooter.PlayerMovement|SetOverlappingLevelEnterOrExit _asbp_player_movement_tutorial false)
      (Variables|Default|Setoverlapping false)
      (Class|PlayerMovement|CallRemovePlayerUIPopupText _asbp_player_movement_tutorial))))

(event Custom|Leave
  (bind _returnvalue (Actor|GetActorOfClass "/Game/Blueprints/Player/BP_PlayerMovement.BP_PlayerMovement_C"))
  (Utilities|Casting|CastToBP_PlayerMovement _returnvalue
    (:then
      (bind _asbp_game_instance (Utilities|Casting|CastToBP_GameInstance (Game|GetGameInstance)))
      (Variables|/Game/Blueprints/BP_GameInstance.BP_GameInstance_C|SetStartingPos _asbp_game_instance "")
      (CallFunction|Exit (Variables|Default|GetLevelToOpen)))
    (:CastFailed
      (bind _returnvalue_2 (Actor|GetActorOfClass "/Game/Blueprints/Tutorial/BP_PlayerMovementTutorial.BP_PlayerMovementTutorial_C"))
      (Utilities|Casting|CastToBP_PlayerMovementTutorial _returnvalue_2)
      (CallFunction|Exit (Variables|Default|GetLevelToOpen)))))

(event EventBeginPlay)

(event Collision|EventActorBeginOverlap
  (params (OtherActor :type Actor%20Object%20Reference)))

(event EventTick
  (params (DeltaSeconds :type Float%20%28single-precision%29))
  (if (Variables|Default|Getoverlapping)
    (bind _returnvalue (Actor|GetActorOfClass "/Game/Blueprints/Player/BP_PlayerMovement.BP_PlayerMovement_C"))
    (bind _asbp_player_movement (Utilities|Casting|CastToBP_PlayerMovement _returnvalue)
      (:then
        (if (Variables|/Script/ExtractShooter.PlayerMovement|GetLeaveLevel _asbp_player_movement)
          (CallFunction|Leave)))
      (:CastFailed
        (bind _returnvalue_2 (Actor|GetActorOfClass "/Game/Blueprints/Tutorial/BP_PlayerMovementTutorial.BP_PlayerMovementTutorial_C"))
        (bind _asbp_player_movement_tutorial (Utilities|Casting|CastToBP_PlayerMovementTutorial _returnvalue_2))
        (if (Variables|/Script/ExtractShooter.PlayerMovement|GetLeaveLevel _asbp_player_movement_tutorial)
          (CallFunction|Leave))))))

(event EventGetBPAudioManager
  (params (BP%20Audio%20Manager :type BP%20Audio%20Manager%20Object%20Reference))
  (Variables|Default|SetBP%20Audio%20Manager BP%20Audio%20Manager))

(event EventExit
  (params (LevelToOpen :type Name :default "None"))
  (bind _returnvalue (Game|GetPlayerCharacter 0))
  (if (not (Variables|Default|GetLock))
    (bind _asbp_game_instance (Utilities|Casting|CastToBP_GameInstance (Game|GetGameInstance)))
    (if (Utilities|String|Contains (Utilities|String|ToString(Name) LevelToOpen) "Tutorial")
      (Default|ClearTutorialInteriorExteriorArrays _asbp_game_instance))
    (Default|ClearLevelManagerArraysandOthers _asbp_game_instance)
    (bind _asbp_player_movement (Utilities|Casting|CastToBP_PlayerMovement _returnvalue)
      (:then
        (Default|SavePlayerStats _asbp_player_movement))
      (:CastFailed
        (Utilities|Casting|CastToBP_PlayerMovementTutorial _returnvalue)))
    (Variables|Default|SetLock true)
    (if (Variables|Default|GetFadeOutAudio)
      (bind _asbp_game_instance_2 (Utilities|Casting|CastToBP_GameInstance (Game|GetGameInstance)))
      (if (Audio|Components|Audio|IsPlaying (Variables|/Game/Blueprints/BP_GameInstance.BP_GameInstance_C|GetBGM%20Playing _asbp_game_instance_2)) :!label _label
        (Audio|Components|Audio|FadeOut (Variables|/Game/Blueprints/BP_GameInstance.BP_GameInstance_C|GetBGM%20Playing _asbp_game_instance_2) (Variables|/Game/Blueprints/Audio/BP_AudioManager.BP_AudioManager_C|GetBGMFadeOutTime (Variables|Default|GetBP%20Audio%20Manager)) 0.0 "Linear" :!class /Script/Engine.AudioComponent)
        (Utilities|FlowControl|DelayUntilNextTick)
        (goto _label)
        (else
          _)))
    (bind _asbp_game_instance_3 (Utilities|Casting|CastToBP_GameInstance (Game|GetGameInstance))
      (:then
        (Variables|/Game/Blueprints/BP_GameInstance.BP_GameInstance_C|SetInLevel _asbp_game_instance_3 false)
        (bind _returnvalue_2 (Game|GetCurrentLevelName true))
        (if (Utilities|String|Contains _returnvalue_2 "Tutorial")
          (Game|OpenLevel(byName) LevelToOpen)
          (else
            (bind _returnvalue_3 (Actor|GetActorOfClass "/Game/Blueprints/UtilityItems/BP_LevelTracker.BP_LevelTracker_C"))
            (bind _levelname (Default|GetRandomLevelName _returnvalue_3 :!label _label_2))
            (if (Utilities|Enum|Equal(Enum) (Utilities|String|ToString(Name) _levelname) "None")
              (Development|PrintString "Level Name Is None, Retrying.... BP Exit")
              (Utilities|FlowControl|Delay 0.2)
              (goto _label_2)
              (else
                (Development|PrintString (Utilities|String|ToString(Name) _levelname))
                (Game|OpenLevel(byName) _levelname))))))
      (:CastFailed
        (Development|PrintString "BP GAME INSTANCE CAST FAILED IN BP EXIT")))))

(fn ConstructionScript)