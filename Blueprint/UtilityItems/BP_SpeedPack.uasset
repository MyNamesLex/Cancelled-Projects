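; BP_SpeedPack is a pickup utility item that carries speed boost duration and intensity for whoever collects it.
; SetItemStats fills in its identity and boost values.
; PickUpItem returns them in a generic item output set shared with weapon and heal fields, with ammo zeroed and ADS off.
; It also calls DestroyItem, which briefly waits, toggles Trigger visibility and teleports the actor below the origin instead of destroying it.
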(event Custom|DestroyItem
  (Utilities|FlowControl|Delay 0.1)
  (Rendering|ToggleVisibility (Variables|Default|GetTrigger) true)
  (Transformation|SetActorLocation "0, 0,-999.000000" false true))

(event EventBeginPlay)

(event Collision|EventActorBeginOverlap
  (params (OtherActor :type Actor%20Object%20Reference)))

(event EventTick
  (params (DeltaSeconds :type Float%20%28single-precision%29)))

(event EventSetItemStats
  (params (Damage :type Integer) (WeaponType :type String) (ItemName :type String) (WeaponRecoil :type Float%20%28double-precision%29) (MagSize :type Integer) (FireRate :type Float%20%28double-precision%29) (ItemType :type String) (SpeedBoostDuration :type String) (SpeedBoostIntensity :type String) (HealIntensity :type String) (HealDuration :type String) (CanADS :type Boolean) (Rifle%20Ammo :type Integer) (Sniper%20Ammo :type Integer) (Shotgun%20Ammo :type Integer) (Pistol%20Ammo :type Integer))
  (Variables|Default|SetItem ItemName)
  (Variables|Default|SetWeaponType WeaponType)
  (Variables|Default|SetItemType ItemType)
  (Variables|Default|SetSpeedBoostDuration SpeedBoostDuration)
  (Variables|Default|SetSpeedBoostIntensity SpeedBoostIntensity))

(fn ConstructionScript)

(fn PickUpItem
  (Development|PrintString "Item Picked Up")
  (CallFunction|DestroyItem)
  (return (Variables|Default|GetItem) (Variables|Default|GetWeaponType) (Variables|Default|GetDamage) (Variables|Default|GetWeaponRecoil) (Variables|Default|GetMagSize) (Variables|Default|GetFireRate) (Variables|Default|GetSpeedPack) (Variables|Default|GetItemType) (Variables|Default|GetSpeedBoostIntensity) (Variables|Default|GetSpeedBoostDuration) (Variables|Default|GetHealIntensity) (Variables|Default|GetHealDuration) false 0 0 0 0))