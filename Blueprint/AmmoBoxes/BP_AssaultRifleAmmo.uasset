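; Assault rifle ammo pickup actor that hands its item stats, including a rifle ammo count, to whatever calls PickUpItem.
; SetItemStats stores the shared weapon and consumable fields but ignores CanADS and non-rifle ammo, which PickUpItem returns as false or zero.
; Pickup prints a message and fires DestroyItem, which after a short delay toggles Trigger visibility and teleports the actor below the map instead of destroying it.
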(event Custom|DestroyItem
  (Utilities|FlowControl|Delay 0.1)
  (Rendering|ToggleVisibility (Variables|Components|GetTrigger) true)
  (Transformation|SetActorLocation "0, 0,-999.000000" false true))

(event EventBeginPlay)

(event Collision|EventActorBeginOverlap
  (params (OtherActor :type Actor%20Object%20Reference)))

(event EventTick
  (params (DeltaSeconds :type Float%20%28single-precision%29)))

(fn ConstructionScript)

(fn PickUpItem
  (Development|PrintString "Item Picked Up")
  (CallFunction|DestroyItem)
  (return (Variables|Default|GetItem) (Variables|Default|GetWeaponType) (Variables|Default|GetDamage) (Variables|Default|GetWeaponRecoil) (Variables|Default|GetMagSize) (Variables|Default|GetFireRate) 0 (Variables|Default|GetItemType) (Variables|Default|GetSpeedBoostIntensity) (Variables|Default|GetSpeedBoostDuration) (Variables|Default|GetHealIntensity) (Variables|Default|GetHealDuration) false (Variables|Default|GetRifle%20Ammo) 0 0 0))

(fn SetItemStats
  (params (Damage :type Integer) (WeaponType :type String) (ItemName :type String) (WeaponRecoil :type Float%20%28double-precision%29) (MagSize :type Integer) (FireRate :type Float%20%28double-precision%29) (ItemType :type String) (SpeedBoostDuration :type String) (SpeedBoostIntensity :type String) (HealIntensity :type String) (HealDuration :type String) (CanADS :type Boolean) (Rifle%20Ammo :type Integer) (Sniper%20Ammo :type Integer) (Shotgun%20Ammo :type Integer) (Pistol%20Ammo :type Integer))
  (Variables|Default|SetDamage Damage)
  (Variables|Default|SetItem ItemName)
  (Variables|Default|SetWeaponType WeaponType)
  (Variables|Default|SetWeaponRecoil WeaponRecoil)
  (Variables|Default|SetMagSize MagSize)
  (Variables|Default|SetFireRate FireRate)
  (Variables|Default|SetItemType ItemType)
  (Variables|Default|SetSpeedBoostIntensity SpeedBoostIntensity)
  (Variables|Default|SetSpeedBoostDuration SpeedBoostDuration)
  (Variables|Default|SetHealIntensity HealIntensity)
  (Variables|Default|SetHealDuration HealDuration)
  (Variables|Default|SetRifle%20Ammo Rifle%20Ammo)
  (return))