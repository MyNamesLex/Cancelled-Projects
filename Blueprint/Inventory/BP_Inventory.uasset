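; Inventory component that passes newly added items, with their weapon, speed boost, heal and ammo stats, to the owning player's inventory widget.
; AddItemToInventory copies its inputs into variables, then calls the widget to add the item to the UI list and store its variables.
; It casts the owner to BP_PlayerMovement, falling back to BP_PlayerMovementTutorial with duplicated calls and printing on each failed cast.
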(event EventBeginPlay)

(event EventTick
  (params (DeltaSeconds :type Float%20%28single-precision%29)))

(fn AddItemtoInventory
  (params (NewItem :type String%20%28by%20ref%29) (NewDamage :type Integer) (NewWeaponType :type String) (NewWeaponRecoil :type Float%20%28double-precision%29) (NewMagSize :type Integer) (NewFireRate :type Float%20%28double-precision%29) (NewStaticMeshComponent :type Static%20Mesh%20Component%20Object%20Reference) (ItemType :type String) (SpeedBoostIntensity :type String) (SpeedBoostDuration :type String) (HealIntensity :type String) (HealDuration :type String) (WeaponCanADS :type Boolean) (Rifle%20Ammo :type Integer) (Sniper%20Ammo :type Integer) (Shotgun%20Ammo :type Integer) (Pistol%20Ammo :type Integer))
  (bind _returnvalue (Components|GetOwner))
  (LocalVariables|Setitem NewItem)
  (LocalVariables|Setdmg NewDamage)
  (LocalVariables|Settype NewWeaponType)
  (LocalVariables|Setrecoil NewWeaponRecoil)
  (LocalVariables|Setmag%20size NewMagSize)
  (LocalVariables|SetFire%20Rate NewFireRate)
  (LocalVariables|Setstatic%20mesh%20component NewStaticMeshComponent)
  (LocalVariables|SetItemTypeLoc ItemType)
  (LocalVariables|SetSpeedBoostIntensityLoc SpeedBoostIntensity)
  (LocalVariables|SetSpeedBoostDurationLoc SpeedBoostDuration)
  (LocalVariables|SetHealIntensityLoc HealIntensity)
  (LocalVariables|SetHealDurationLoc HealDuration)
  (LocalVariables|Setads WeaponCanADS)
  (LocalVariables|Setrammo Rifle%20Ammo)
  (LocalVariables|SetSniperammo Sniper%20Ammo)
  (LocalVariables|SetShotgunAmmo Shotgun%20Ammo)
  (LocalVariables|SetPammo Pistol%20Ammo)
  (bind _asbp_player_movement (Utilities|Casting|CastToBP_PlayerMovement _returnvalue)
    (:then
      (Default|AddItemtoInventoryUILIst (Variables|/Game/Blueprints/Player/BP_PlayerMovement.BP_PlayerMovement_C|GetInventoryWidget _asbp_player_movement) (LocalVariables|Getitem) (LocalVariables|Getdmg) (LocalVariables|Gettype) (LocalVariables|Getrecoil) (LocalVariables|Getmag%20size) (LocalVariables|GetFire%20Rate) (LocalVariables|Getstatic%20mesh%20component) (LocalVariables|GetItemTypeLoc) (LocalVariables|GetSpeedBoostIntensityLoc) (LocalVariables|GetSpeedBoostDurationLoc) (LocalVariables|GetHealIntensityLoc) (LocalVariables|GetHealDurationLoc) (LocalVariables|Getads) (LocalVariables|GetShotgunAmmo) (LocalVariables|GetPammo) (LocalVariables|GetSniperammo) (LocalVariables|Getrammo))
      (Default|StoreItemVariables (Variables|/Game/Blueprints/Player/BP_PlayerMovement.BP_PlayerMovement_C|GetInventoryWidget _asbp_player_movement) (LocalVariables|Gettype) (LocalVariables|Getitem) (LocalVariables|Getdmg) (LocalVariables|Getrecoil) (LocalVariables|Getmag%20size) (LocalVariables|GetFire%20Rate) (LocalVariables|Getstatic%20mesh%20component) (LocalVariables|GetItemTypeLoc) (LocalVariables|GetSpeedBoostIntensityLoc) (LocalVariables|GetSpeedBoostDurationLoc) (LocalVariables|GetHealIntensityLoc) (LocalVariables|GetHealDurationLoc) (LocalVariables|Getads) (LocalVariables|GetSniperammo) (LocalVariables|GetShotgunAmmo) (LocalVariables|GetPammo) (LocalVariables|Getrammo)))
    (:CastFailed
      (Development|PrintString "FAILED PLAYER CAST BP INVENTORY")
      (bind _asbp_player_movement_tutorial (Utilities|Casting|CastToBP_PlayerMovementTutorial _returnvalue)
        (:then
          (Default|AddItemtoInventoryUILIst (Variables|/Game/Blueprints/Tutorial/BP_PlayerMovementTutorial.BP_PlayerMovementTutorial_C|GetInventoryWidget _asbp_player_movement_tutorial) (LocalVariables|Getitem) (LocalVariables|Getdmg) (LocalVariables|Gettype) (LocalVariables|Getrecoil) (LocalVariables|Getmag%20size) (LocalVariables|GetFire%20Rate) (LocalVariables|Getstatic%20mesh%20component) (LocalVariables|GetItemTypeLoc) (LocalVariables|GetSpeedBoostIntensityLoc) (LocalVariables|GetSpeedBoostDurationLoc) (LocalVariables|GetHealIntensityLoc) (LocalVariables|GetHealDurationLoc) (LocalVariables|Getads) (LocalVariables|GetShotgunAmmo) (LocalVariables|GetPammo) (LocalVariables|GetSniperammo) (LocalVariables|Getrammo))
          (Default|StoreItemVariables (Variables|/Game/Blueprints/Tutorial/BP_PlayerMovementTutorial.BP_PlayerMovementTutorial_C|GetInventoryWidget _asbp_player_movement_tutorial) (LocalVariables|Gettype) (LocalVariables|Getitem) (LocalVariables|Getdmg) (LocalVariables|Getrecoil) (LocalVariables|Getmag%20size) (LocalVariables|GetFire%20Rate) (LocalVariables|Getstatic%20mesh%20component) (LocalVariables|GetItemTypeLoc) (LocalVariables|GetSpeedBoostIntensityLoc) (LocalVariables|GetSpeedBoostDurationLoc) (LocalVariables|GetHealIntensityLoc) (LocalVariables|GetHealDurationLoc) (LocalVariables|Getads) (LocalVariables|GetSniperammo) (LocalVariables|GetShotgunAmmo) (LocalVariables|GetPammo) (LocalVariables|Getrammo)))
        (:CastFailed
          (Development|PrintString "FAILED PLAYER TUTORIAL CAST BP INVENTORY"))))))