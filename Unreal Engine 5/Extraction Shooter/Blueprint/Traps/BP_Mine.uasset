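; Mine trap for an extraction shooter that explodes once, on a hit or an Explode call.
; Detonation traces for a surface material to feed the Niagara effects, hides the mine and briefly enables radius overlap events.
; Overlapped AI and players are stunned and take damage computed from the mine-to-radius-component distance plus a base amount.
; The overlap handler also plays explosion and ear-ringing sounds through the audio manager, then destroys the actor.
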(event OnComponentHit(Mine)
  (params (HitComponent :type Primitive%20Component%20Object%20Reference) (OtherActor :type Actor%20Object%20Reference) (OtherComp :type Primitive%20Component%20Object%20Reference) (NormalImpulse :type Vector :default "0, 0, 0") (Hit :type Hit%20Result%20Structure%20%28by%20ref%29))
  (CallFunction|ExplodeFunc))

(event OnComponentBeginOverlap(ExplosionRadius)
  (params (OverlappedComponent :type Primitive%20Component%20Object%20Reference) (OtherActor :type Actor%20Object%20Reference) (OtherComp :type Primitive%20Component%20Object%20Reference) (OtherBodyIndex :type Integer) (bFromSweep :type Boolean) (SweepResult :type Hit%20Result%20Structure%20%28by%20ref%29))
  (bind _returnvalue (Transformation|GetWorldLocation OverlappedComponent))
  (bind _bp_audio_manager (Variables|Default|GetBP%20Audio%20Manager))
  (bind _mine (Variables|Default|GetMine))
  (bind _returnvalue_2 (Transformation|GetWorldLocation _mine))
  (bind _returnvalue_3 (- _returnvalue_2 _returnvalue))
  (bind _returnvalue_4 (Math|Vector|VectorLength _returnvalue_3))
  (bind _returnvalue_5 (+ _returnvalue_4 25.0))
  (bind _asbp_aiinterface (Utilities|Casting|CastToBP_AIInterface OtherActor)
    (:then
      (Default|DamageDeal _asbp_aiinterface (Math|Float|Truncate _returnvalue_5))
      (Default|Stunned _asbp_aiinterface))
    (:CastFailed
      _))
  (bind _asbp_player_movement (Utilities|Casting|CastToBP_PlayerMovement OtherActor)
    (:then
      (Class|PlayerMovement|DealDamagetoPlayer _asbp_player_movement _returnvalue_5)
      (Default|StunnedFunc _asbp_player_movement))
    (:CastFailed
      _))
  (Variables|/Script/Engine.PrimitiveComponent|SetbGenerateOverlapEvents (Variables|Default|GetExplosionRadius) true)
  (Default|PlaySFXbyName _bp_audio_manager "Explosion" (Transformation|GetActorLocation _asbp_player_movement))
  (Default|PlaySFXbyName _bp_audio_manager "RingingEars" (Transformation|GetActorLocation _asbp_player_movement))
  (Actor|DestroyActor))

(event Custom|Explode%20Func
  (bind _mine (Variables|Default|GetMine))
  (bind _explosionradius (Variables|Default|GetExplosionRadius))
  (if (not (Variables|Default|GetTriggered))
    (Variables|Default|SetTriggered true)
    (bind _outhit (Collision|LineTraceByChannel (Transformation|GetWorldLocation (Variables|Default|GetMine)) "0, 0,99.000000" "TraceTypeQuery1" false 0 "None"))
    (bind _output_get (Variables|Default|SetGroundMat (Rendering|Material|GetMaterial (.HitComponent (Collision|BreakHitResult _outhit)) 0)))
    (bind _output_get_2 (Variables|Default|SetParticleComponent (Variables|Default|GetNiagara)))
    (Class|NiagaraComponent|SetVariableMaterial _output_get_2 "GroundMat" _output_get)
    (Variables|Default|SetOuterClaymoreExplosion (Variables|Default|GetOuterClaymoreParticles))
    (Variables|Default|SetInnerClaymoreExplosion (Variables|Default|GetInnerClaymoreParticles))
    (Class|Claymore|Explosion)
    (Rendering|SetVisibility _mine false false)
    (Collision|SetCollisionEnabled _mine "NoCollision")
    (Variables|/Script/Engine.PrimitiveComponent|SetbGenerateOverlapEvents _explosionradius true)
    (Utilities|FlowControl|Delay 0.2)
    (Variables|/Script/Engine.PrimitiveComponent|SetbGenerateOverlapEvents _explosionradius false)))

(event EventBeginPlay)

(event Collision|EventActorBeginOverlap
  (params (OtherActor :type Actor%20Object%20Reference)))

(event EventTick
  (params (DeltaSeconds :type Float%20%28single-precision%29)))

(event EventExplode
  (CallFunction|ExplodeFunc))

(event EventGetBPAudioManager
  (params (BP%20Audio%20Manager :type BP%20Audio%20Manager%20Object%20Reference))
  (Variables|Default|SetBP%20Audio%20Manager BP%20Audio%20Manager))

(fn ConstructionScript)