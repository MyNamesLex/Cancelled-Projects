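; Gate exit actor that lets the player leave the level for a configured level.
; Cube overlap toggles a "Leave Level?" popup, and Tick polls LeaveLevel on the regular or tutorial player while overlapping.
; Leave clears GameInstance state and saves stats; Exit freezes AI, optionally wipes inventory, then opens LevelToOpen.
; Saving and exiting require BP_PlayerMovement, so the tutorial character's path stops at that cast.
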(event OnComponentBeginOverlap(Cube)
  (params (OverlappedComponent :type Primitive%20Component%20Object%20Reference) (OtherActor :type Actor%20Object%20Reference) (OtherComp :type Primitive%20Component%20Object%20Reference) (OtherBodyIndex :type Integer) (bFromSweep :type Boolean) (SweepResult :type Hit%20Result%20Structure%20%28by%20ref%29))
  (bind _asbp_player_movement (Utilities|Casting|CastToBP_PlayerMovement OtherActor)
    (:then
      (Variables|/Script/ExtractShooter.PlayerMovement|SetOverlappingLevelEnterOrExit _asbp_player_movement true)
      (Variables|Default|Setoverlapping true)
      (Class|PlayerMovement|CallPlayerUIPopupText _asbp_player_movement "Leave Level? \"L\"" 1e+69))
    (:CastFailed
      (bind _asbp_player_movement_tutorial (Utilities|Casting|CastToBP_PlayerMovementTutorial OtherActor))
      (Variables|/Script/ExtractShooter.PlayerMovement|SetOverlappingLevelEnterOrExit _asbp_player_movement_tutorial true)
      (Variables|Default|Setoverlapping true)
      (Class|PlayerMovement|CallPlayerUIPopupText _asbp_player_movement_tutorial "Leave Level? \"L\"" 1e+69))))

(event OnComponentEndOverlap(Cube)
  (params (OverlappedComponent :type Primitive%20Component%20Object%20Reference) (OtherActor :type Actor%20Object%20Reference) (OtherComp :type Primitive%20Component%20Object%20Reference) (OtherBodyIndex :type Integer))
  (bind _asbp_player_movement (Utilities|Casting|CastToBP_PlayerMovement OtherActor)
    (:then
      (Variables|/Script/ExtractShooter.PlayerMovement|SetOverlappingLevelEnterOrExit _asbp_player_movement false)
      (Variables|Default|Setoverlapping false)
      (Class|PlayerMovement|CallRemovePlayerUIPopupText _asbp_player_movement))
    (:CastFailed
      (bind _asbp_player_movement_tutorial (Utilities|Casting|CastToBP_PlayerMovementTutorial OtherActor))
      (Variables|/Script/ExtractShooter.PlayerMovement|SetOverlappingLevelEnterOrExit _asbp_player_movement_tutorial false)
      (Variables|Default|Setoverlapping false)
      (Class|PlayerMovement|CallRemovePlayerUIPopupText _asbp_player_movement_tutorial))))

(event Custom|Leave
  (bind _asbp_game_instance (Utilities|Casting|CastToBP_GameInstance (Game|GetGameInstance)))
  (Default|ClearTutorialInteriorExteriorArrays _asbp_game_instance)
  (Variables|/Game/Blueprints/BP_GameInstance.BP_GameInstance_C|SetStartingPos _asbp_game_instance "")
  (bind _asbp_player_movement (Utilities|Casting|CastToBP_PlayerMovement (Game|GetPlayerCharacter 0)))
  (Default|SavePlayerStats _asbp_player_movement)
  (CallFunction|Exit (Variables|Default|GetLevelToOpen)))

(event EventBeginPlay)

(event EventTick
  (params (DeltaSeconds :type Float%20%28single-precision%29))
  (if (Variables|Default|Getoverlapping)
    (bind _returnvalue (Actor|GetActorOfClass "/Game/Blueprints/Player/BP_PlayerMovement.BP_PlayerMovement_C"))
    (bind _asbp_player_movement (Utilities|Casting|CastToBP_PlayerMovement _returnvalue)
      (:then
        (if (Variables|/Script/ExtractShooter.PlayerMovement|GetLeaveLevel _asbp_player_movement)
          (CallFunction|Leave)))
      (:CastFailed
        (bind _returnvalue_2 (Actor|GetActorOfClass "/Game/Blueprints/Tutorial/BP_PlayerMovementTutorial.BP_PlayerMovementTutorial_C"))
        (bind _asbp_player_movement_tutorial (Utilities|Casting|CastToBP_PlayerMovementTutorial _returnvalue_2))
        (if (Variables|/Script/ExtractShooter.PlayerMovement|GetLeaveLevel _asbp_player_movement_tutorial)
          (CallFunction|Leave))))))

(event EventExit
  (params (LevelToOpen :type Name :default "None"))
  (bind _asbp_player_movement (Utilities|Casting|CastToBP_PlayerMovement (Game|GetPlayerCharacter 0)))
  (Variables|Default|SetBP%20Player _asbp_player_movement)
  (Default|FreezeAI _asbp_player_movement)
  (bind _asbp_game_instance (Utilities|Casting|CastToBP_GameInstance (Game|GetGameInstance))
    (:then
      (Default|ClearTutorialInteriorExteriorArrays _asbp_game_instance)
      (Default|ClearLevelManagerArraysandOthers _asbp_game_instance)
      (if (Variables|Default|GetWipeInventory)
        (if (Variables|/Script/ExtractShooter.PlayerMovement|GetinInventory (Variables|Default|GetBP%20Player))
          (Default|ToggleInventory (Variables|Default|GetBP%20Player))
          (Utilities|FlowControl|Delay 0.2))
        (Default|RemoveEverythingfromInventory (Variables|Default|GetBP%20Player))
        (Utilities|FlowControl|Delay 0.2)
        (Default|RemoveEverythingfromInventory (Variables|Default|GetBP%20Player))
        (Default|RemoveEverythingfromInventory (Variables|Default|GetBP%20Player)))
      (Game|OpenLevel(byName) LevelToOpen))
    (:CastFailed
      (Development|PrintString "BP GAME INSTANCE CAST FAILED IN BP EXIT"))))

(fn ConstructionScript)