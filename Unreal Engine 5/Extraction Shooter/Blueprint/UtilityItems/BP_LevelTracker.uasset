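; BP_LevelTracker is an actor that chooses the next level name from the player's completed-level count in BP_GameInstance.
; GetRandomLevelName draws from the normal list, or from the hard list on a chance roll past a threshold; a failed roll has no selection path.
; Exact milestone counts override the pick with first boss, second boss or random ending levels.
; A valid pick increments the count immediately, before returning.
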(event EventBeginPlay)

(event Collision|EventActorBeginOverlap
  (params (OtherActor :type Actor%20Object%20Reference)))

(event EventTick
  (params (DeltaSeconds :type Float%20%28single-precision%29)))

(fn ConstructionScript)

(fn GetRandomLevelName
  (bind _asbp_game_instance (Utilities|Casting|CastToBP_GameInstance (Game|GetGameInstance)))
  (if (>= (Variables|/Game/Blueprints/BP_GameInstance.BP_GameInstance_C|GetPlayerLevelsDone _asbp_game_instance) (Variables|Default|GetStartHardLevels))
    (if (<= (Math|Random|RandomIntegerinRange 0 100) (Variables|Default|GetHardLevelChance))
      (bind _levelname (CallFunction|GetRandomHardLevelName))
      (Variables|Default|SetLevelName _levelname)
      (bind _asbp_game_instance_2 (Utilities|Casting|CastToBP_GameInstance (Game|GetGameInstance) :!label _label))
      (if (== (Variables|/Game/Blueprints/BP_GameInstance.BP_GameInstance_C|GetPlayerLevelsDone _asbp_game_instance_2) (Variables|Default|GetFirstBossLevelStart))
        (bind _level_name (CallFunction|FirstBossLevelName))
        (Variables|Default|SetLevelName _level_name))
      (bind _asbp_game_instance_3 (Utilities|Casting|CastToBP_GameInstance (Game|GetGameInstance)))
      (if (== (Variables|/Game/Blueprints/BP_GameInstance.BP_GameInstance_C|GetPlayerLevelsDone _asbp_game_instance_3) (Variables|Default|GetSecondBossLevelStart))
        (bind _level_name_2 (CallFunction|SecondBossLevelName))
        (Variables|Default|SetLevelName _level_name_2))
      (bind _asbp_game_instance_4 (Utilities|Casting|CastToBP_GameInstance (Game|GetGameInstance)))
      (if (== (Variables|Default|GetEndingLevelStart) (Variables|/Game/Blueprints/BP_GameInstance.BP_GameInstance_C|GetPlayerLevelsDone _asbp_game_instance_4))
        (bind _levelname_2 (CallFunction|GetEndingLevelName))
        (Variables|Default|SetLevelName _levelname_2))
      (if (Utilities|Enum|Equal(Enum) (Utilities|String|ToString(Name) (Variables|Default|GetLevelName)) "None")
        _
        (else
          (bind _asbp_game_instance_5 (Utilities|Casting|CastToBP_GameInstance (Game|GetGameInstance)))
          (Variables|/Game/Blueprints/BP_GameInstance.BP_GameInstance_C|SetPlayerLevelsDone _asbp_game_instance_5 (+ (Variables|/Game/Blueprints/BP_GameInstance.BP_GameInstance_C|GetPlayerLevelsDone _asbp_game_instance_5) 1))))
      (return (Variables|Default|GetLevelName)))
    (else
      (Variables|Default|SetLevelName (Utilities|Array|Get(acopy) (Variables|Default|GetLevelNameList) (Math|Random|RandomIntegerinRange 0 (- (Utilities|Array|Length (Variables|Default|GetLevelNameList)) 1))))
      (goto _label))))

(fn GetRandomHardLevelName
  (return (Utilities|Array|Get(acopy) (Variables|Default|GetHardLevelNameList) (Math|Random|RandomIntegerinRange 0 (- (Utilities|Array|Length (Variables|Default|GetHardLevelNameList)) 1)))))

(fn GetEndingLevelName
  (return (Utilities|Array|Get(acopy) (Variables|Default|GetEndingLevelNameList) (Math|Random|RandomIntegerinRange 0 (- (Utilities|Array|Length (Variables|Default|GetEndingLevelNameList)) 1)))))

(fn FirstBossLevelName
  (return (Variables|Default|GetFirstBossLevel)))

(fn SecondBossLevelName
  (return (Variables|Default|GetSecondBossLevel)))