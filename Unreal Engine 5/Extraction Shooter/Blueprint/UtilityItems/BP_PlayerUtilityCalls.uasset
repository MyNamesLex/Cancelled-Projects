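; Utility actor that clears the player's inventory or removes a single item from it by index.
; It caches BP_PlayerMovement and its InventoryWidget on BeginPlay, then removes list entries and their stored widget data.
; Full clears also edit the player's ItemArray and refresh ammo UI and weapon stats, while single removals refresh weapon stats and fix sorting.
; Failed widget removals retry after a short delay.
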(event Custom|RemoveItemFromInventory
  (params (Index :type Integer))
  (bind _inventory_widget (Variables|Default|GetInventory%20Widget))
  (bind _listvertical (Variables|/Game/Blueprints/Inventory/BP_InventoryWidget.BP_InventoryWidget_C|GetListVertical _inventory_widget))
  (bind _returnvalue (Class|PanelWidget|GetAllChildren _listvertical))
  (bind _output (Utilities|Array|Get(acopy) _returnvalue Index))
  (Development|PrintString "REMOVE ITEM FROM INVENTORY CALLED")
  (Default|RemoveStoredItemVarsinArrays _inventory_widget Index)
  (Utilities|Array|RemoveItem _returnvalue _output)
  (bind _returnvalue_2 (Class|PanelWidget|RemoveChild _listvertical _output :!label _label))
  (if _returnvalue_2
    (Default|GetCurrentWeaponStats (Variables|Default|GetBP%20Player))
    (Default|FixInventorySorting _inventory_widget)
    (Development|PrintString "ITEM REMOVED")
    (else
      (Development|PrintString "ITEM NOT REMOVED")
      (Utilities|FlowControl|Delay 0.2)
      (goto _label))))

(event Custom|RemoveEverythingFromInventory
  (if (== (Variables|Default|GetInventory%20Widget) 0) :!label _label
    (bind _asbp_player_movement (Utilities|Casting|CastToBP_PlayerMovement (Game|GetPlayerCharacter 0))
      (:then
        (bind _output_get (Variables|Default|SetBP%20Player _asbp_player_movement))
        (Variables|Default|SetInventory%20Widget (Variables|/Game/Blueprints/Player/BP_PlayerMovement.BP_PlayerMovement_C|GetInventoryWidget _output_get))
        (goto _label))
      (:CastFailed
        (Development|PrintString "CAST TO PLAYER FAILED BP PLAYERUTILITYCALLS")))
    (else
      (Development|PrintString "REMOVE EVERYTHING FROM INVENTORY CALLED")
      (for (_array_element _array_index) (Class|PanelWidget|GetAllChildren (Variables|/Game/Blueprints/Inventory/BP_InventoryWidget.BP_InventoryWidget_C|GetListVertical (Variables|Default|GetInventory%20Widget))) :!label _label_2
        (bind _returnvalue (Class|PanelWidget|RemoveChild (Variables|/Game/Blueprints/Inventory/BP_InventoryWidget.BP_InventoryWidget_C|GetListVertical (Variables|Default|GetInventory%20Widget)) _array_element))
        (Default|RemoveStoredItemVarsinArrays (Variables|Default|GetInventory%20Widget) _array_index)
        (Utilities|Array|RemoveItem (Variables|/Game/Blueprints/Player/BP_PlayerMovement.BP_PlayerMovement_C|GetItemArray (Variables|Default|GetBP%20Player)) (Utilities|Array|Get(acopy) (Variables|/Game/Blueprints/Player/BP_PlayerMovement.BP_PlayerMovement_C|GetItemArray (Variables|Default|GetBP%20Player)) _array_index))
        (if _returnvalue
          (Class|PlayerMovement|UpdatePlayerAmmoonUI (Variables|Default|GetBP%20Player))
          (Default|GetCurrentWeaponStats (Variables|Default|GetBP%20Player))
          (Development|PrintString "ITEM REMOVED")
          (else
            (Development|PrintString "ITEM NOT REMOVED")
            (Utilities|FlowControl|Delay 0.2)
            (goto _label_2))))
      (Development|PrintString "INVENTORY CLEARED"))))

(event EventBeginPlay
  (bind _asbp_player_movement (Utilities|Casting|CastToBP_PlayerMovement (Game|GetPlayerCharacter 0))
    (:then
      (bind _output_get (Variables|Default|SetBP%20Player _asbp_player_movement))
      (Variables|Default|SetInventory%20Widget (Variables|/Game/Blueprints/Player/BP_PlayerMovement.BP_PlayerMovement_C|GetInventoryWidget _output_get)))
    (:CastFailed
      (Development|PrintString "CAST TO PLAYER FAILED BP PLAYERUTILITYCALLS"))))

(event Collision|EventActorBeginOverlap
  (params (OtherActor :type Actor%20Object%20Reference)))

(event EventTick
  (params (DeltaSeconds :type Float%20%28single-precision%29)))

(fn ConstructionScript)