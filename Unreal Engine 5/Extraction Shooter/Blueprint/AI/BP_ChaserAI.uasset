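; Chaser enemy AI that roams to random points, pursues the player on sight or perception stimulus, and deals melee damage while its hitbox overlaps them.
; PawnSensing and AIPerception drive AIMoveTo chases, with a retriggerable delay clearing player awareness after sight-based chases.
; Tick drives wandering and delayed hits, gated by active and dead flags.
; It supports stun slowdown and toggling, and reports its death to BP_InteriorEntranceManager by tag.
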(event OnTargetPerceptionUpdated(AIPerception)
  (params (Actor :type Actor%20Object%20Reference) (Stimulus :type AI%20Stimulus%20Structure))
  (if (Variables|Default|GetisActive)
    (if (not (Variables|Default|GetDeadBool))
      (Development|PrintString "AI Heard Sound")
      (CallFunction|SeePlayer))))

(event OnSeePawn(PawnSensing)
  (params (Pawn :type Pawn%20Object%20Reference))
  (if (Variables|Default|GetisActive)
    (if (Variables|Default|GetCanSeePlayer)
      _
      (else
        (Utilities|FlowControl|Delay (Variables|Default|GetSeePlayerDelay))))
    (CallFunction|ChasePlayer Pawn)))

(event OnComponentBeginOverlap(HitBox)
  (params (OverlappedComponent :type Primitive%20Component%20Object%20Reference) (OtherActor :type Actor%20Object%20Reference) (OtherComp :type Primitive%20Component%20Object%20Reference) (OtherBodyIndex :type Integer) (bFromSweep :type Boolean) (SweepResult :type Hit%20Result%20Structure%20%28by%20ref%29))
  ;[1 1 1] Damage / Deal Damage
  (if (not (Variables|Default|GetDeadBool))
    (bind _asbp_player_movement (Utilities|Casting|CastToBP_PlayerMovement OtherActor))
    (if (Variables|/Script/ExtractShooter.PlayerMovement|GetDead _asbp_player_movement)
      (Variables|Default|SetDealDamage false)
      (elif (Collision|IsOverlappingActor (Variables|/Script/Engine.Character|GetMesh _asbp_player_movement) self :!class /Script/Engine.PrimitiveComponent)
        (bind _output_get (Variables|Default|SetPlayer _asbp_player_movement))
        (Variables|Default|SetDealDamage true)
        (AI|AIMoveTo self (Transformation|GetActorLocation _output_get) _asbp_player_movement 0.0 false)))))

(event OnComponentEndOverlap(HitBox)
  (params (OverlappedComponent :type Primitive%20Component%20Object%20Reference) (OtherActor :type Actor%20Object%20Reference) (OtherComp :type Primitive%20Component%20Object%20Reference) (OtherBodyIndex :type Integer))
  ;[1 1 1] Damage / Deal Damage
  (Utilities|Casting|CastToBP_PlayerMovement OtherActor)
  (Variables|Default|SetDealDamage false))

(event Custom|Dead
  ;[1 1 1] Damage / Deal Damage
  (Development|PrintString "Dead")
  (Variables|Default|SetDeadBool true)
  (Components|Animation|PlayAnimation (Variables|Character|GetMesh) "/Game/Assets/Models/Player/Dead/Falling_Forward_Death_Anim_mixamo_com.Falling_Forward_Death_Anim_mixamo_com" false)
  (CallFunction|ToggleAIFunctionality false)
  (bind _returnvalue (Actor|GetActorOfClass "/Game/Blueprints/UtilityItems/BP_InteriorEntranceManager.BP_InteriorEntranceManager_C"))
  (bind _asbp_interior_entrance_manager (Utilities|Casting|CastToBP_InteriorEntranceManager _returnvalue))
  (Default|SetDeadEnemiesFunc _asbp_interior_entrance_manager (Utilities|Array|Get(acopy) (Variables|Actor|GetTags self))))

(event Custom|DealDamageFunc
  (params (Player :type BP%20Player%20Movement%20Object%20Reference))
  ;[1 1 1] Damage / Deal Damage
  (if (Variables|/Script/ExtractShooter.PlayerMovement|GetDead Player)
    (Variables|Default|SetDealDamage false)
    (else
      (Variables|Default|SetCanSeePlayer true)
      (Development|PrintString "Enemy AI Hit Player")
      (Class|PlayerMovement|DealDamagetoPlayer Player (Variables|Default|GetDamage)))))

(event Custom|Chase%20Player
  (params (Pawn :type Pawn%20Object%20Reference))
  (if (Variables|Default|GetisActive)
    (if (not (Variables|Default|GetDeadBool))
      (Utilities|Casting|CastToBP_PlayerMovement Pawn)
      (Utilities|FlowControl|Sequence
        (:then_0
          (if (Variables|Default|GetisActive)
            (CallFunction|SeePlayer)))
        (:then_1
          (if (Variables|Default|GetisActive)
            ;[1 1 1] Doesnt See Player
            (Utilities|FlowControl|RetriggerableDelay (Variables|Default|GetMemory))
            (Variables|Default|SetCanSeePlayer false)))))))

(event Custom|See%20Player
  ;[1 1 1] Chase Player As Soon As AI Sees Player
  (Variables|Default|SetCanSeePlayer true)
  (bind _asbp_player_movement (Utilities|Casting|CastToBP_PlayerMovement (Game|GetPlayerCharacter 0)))
  (AI|AIMoveTo self (Transformation|GetActorLocation _asbp_player_movement) 0 5.0 false))

(event EventStunned
  (bind _charactermovement (Variables|Character|GetCharacterMovement))
  (Variables|/Script/Engine.CharacterMovementComponent|SetMaxWalkSpeed _charactermovement 5e+01)
  (Utilities|FlowControl|Delay 5.0)
  (Variables|/Script/Engine.CharacterMovementComponent|SetMaxWalkSpeed _charactermovement 6e+02))

(event EventToggleAIFunctionality
  (params (Active :type Boolean))
  (Variables|Default|SetisActive Active)
  (Components|Movement|StopMovementImmediately (Variables|Character|GetCharacterMovement))
  (Class|NavMovementComponent|StopActiveMovement (Variables|Character|GetCharacterMovement)))

(event EventTick
  (params (DeltaSeconds :type Float%20%28single-precision%29))
  ;[1 1 1] Deal Melee Damage Check
  (if (Variables|Default|GetisActive)
    (if (not (Variables|Default|GetDeadBool))
      (if (Variables|Default|GetDealDamage)
        (Utilities|FlowControl|Delay 0.2)
        (CallFunction|DealDamageFunc (Variables|Default|GetPlayer))
        (else
          ;[1 1 1] Wait A Random Amount Of Time
          (if (not (Variables|Default|GetCanSeePlayer))
            (Utilities|FlowControl|Delay (Math|Random|RandomFloatinRange 2.0 4.0))
            ;[1 1 1] Move AI To A Random Location Within A Radius Of 4000 From Itself
            (if (Variables|Default|GetisActive)
              (AI|AIMoveTo self (.RandomLocation (AI|Navigation|GetRandomReachablePointinRadius (Transformation|GetActorLocation) 4e+03 0 0)) 0 5.0 true
                (:then
                  (Variables|Default|SetIsMoving true))
                (:OnSuccess
                  (Variables|Default|SetIsMoving false))))))))))

(event EventSetSpeed
  (params (Speed :type Float%20%28double-precision%29))
  (Variables|/Script/Engine.CharacterMovementComponent|SetMaxWalkSpeed (Variables|Character|GetCharacterMovement) Speed))

(event EventFindPlayer
  (CallFunction|ChasePlayer (Game|Player|GetPlayerPawn 0)))

(event EventGetBPAudioManager
  (params (BP%20Audio%20Manager :type BP%20Audio%20Manager%20Object%20Reference))
  (Variables|Default|SetBP%20Audio%20Manager BP%20Audio%20Manager))

(fn ConstructionScript)

(fn DamageDeal
  (params (Damage :type Integer))
  (if (not (Variables|Default|GetDeadBool))
    (Variables|Default|SetHealth (- (Variables|Default|GetHealth) Damage))
    (if (<= (Variables|Default|GetHealth) 0.0)
      (CallFunction|Dead))))

(fn GetHealth
  (return (Variables|Default|GetHealth)))