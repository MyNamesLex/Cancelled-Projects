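; Level dialogue actor that plays named lines in BP_DialogueWidget with a character-by-character typewriter effect and per-line popup text.
; On BeginPlay it starts gameplay dialogue, gated by GameInstance play-once flags, or readies cutscene dialogue after fade-out.
; NextDialogueNoCutscene advances lines, optionally freezing player and AI.
; Completion triggers a level exit or level load, or clears the UI, unfreezes and hands off to any chained dialogue.
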(event Custom|EndDialogue
  (bind _bp_player_movement (Variables|Default|GetBP%20Player%20Movement))
  (bind _bp_dialogue_widget (Variables|Default|GetBP%20Dialogue%20Widget))
  (bind _bp_dialogue_widget_2 (Variables|Default|GetBP%20Dialogue%20Widget))
  (bind _playerui (Variables|/Game/Blueprints/Player/BP_PlayerMovement.BP_PlayerMovement_C|GetPlayerUI _bp_player_movement))
  (bind _asbp_game_instance (Utilities|Casting|CastToBP_GameInstance (Game|GetGameInstance)))
  (Variables|/Game/Blueprints/BP_GameInstance.BP_GameInstance_C|SetHasPlayedDialogue _asbp_game_instance true)
  (Variables|Default|SetLockDialogue true)
  (Rendering|Components|TextRender|SetText (Variables|/Game/Blueprints/UI/BP_DialogueWidget.BP_DialogueWidget_C|GetNameText _bp_dialogue_widget_2) "")
  (Rendering|Components|TextRender|SetText (Variables|/Game/Blueprints/UI/BP_DialogueWidget.BP_DialogueWidget_C|GetDialogueText _bp_dialogue_widget_2) "")
  (Rendering|Components|TextRender|SetText (Variables|/Game/Blueprints/UI/BP_PlayerUI.BP_PlayerUI_C|GetPopupTextUI _playerui) "")
  (Class|Image|SetOpacity (Variables|/Game/Blueprints/UI/BP_DialogueWidget.BP_DialogueWidget_C|GetNameImage _bp_dialogue_widget) 0.0)
  (Class|Image|SetOpacity (Variables|/Game/Blueprints/UI/BP_DialogueWidget.BP_DialogueWidget_C|GetDialogueImage _bp_dialogue_widget) 0.0)
  (Class|TextBlock|SetOpacity (Variables|/Game/Blueprints/UI/BP_DialogueWidget.BP_DialogueWidget_C|GetContinueText (Variables|Default|GetBP%20Dialogue%20Widget)) 0.0)
  (Class|Image|SetOpacity (Variables|/Game/Blueprints/UI/BP_PlayerUI.BP_PlayerUI_C|GetPopupTextImage _playerui) 0.0)
  (Widget|RemovefromParent (Variables|Default|GetBP%20Dialogue%20Widget))
  (if (not (== (Variables|Default|GetNextDialogueToPlay) 0))
    (Variables|/Game/Blueprints/Player/BP_PlayerMovement.BP_PlayerMovement_C|SetBP%20Dialogue (Variables|Default|GetBP%20Player%20Movement) (Variables|Default|GetNextDialogueToPlay))
    (Utilities|FlowControl|Delay 0.2)
    (Actor|DestroyActor)))

(event Custom|NextDialogueNoCutscene
  (bind _dialogue (Variables|Default|GetDialogue))
  (bind _nextscenename (Variables|Default|GetNextSceneName))
  (if (Variables|Default|GetFreezeAIUntilAfterDialogue)
    (Default|FreezeAI (Variables|Default|GetBP%20Player%20Movement)))
  (if (Variables|Default|GetFreezePlayerUntilAfterDialogue)
    (Default|FreezePlayer (Variables|Default|GetBP%20Player%20Movement)))
  (if (== (Variables|Default|GetBP%20Dialogue%20Widget) 0) :!label _label
    (bind _returnvalue (UserInterface|CreateWidget "/Game/Blueprints/UI/BP_DialogueWidget.BP_DialogueWidget_C"))
    (bind _output_get (Variables|Default|SetBP%20Dialogue%20Widget _returnvalue))
    (UserInterface|Viewport|AddtoViewport _output_get 0)
    (Utilities|FlowControl|Delay 0.2)
    (goto _label)
    (else
      (Class|TextBlock|SetOpacity (Variables|/Game/Blueprints/UI/BP_DialogueWidget.BP_DialogueWidget_C|GetContinueText (Variables|Default|GetBP%20Dialogue%20Widget)) 1.0)
      (Development|PrintString "next dialogue")
      (bind _output_get_2 (Variables|Default|SetNameStr (Utilities|Array|Get(acopy) (Variables|Default|GetName) (Variables|Default|GetCounter))))
      (bind _output_get_3 (Variables|Default|SetDialogueStr (Utilities|Array|Get(acopy) _dialogue (Variables|Default|GetCounter))))
      (CallFunction|PlaceImagesinWidget _output_get_2 _output_get_3)
      (if (>= (Variables|Default|GetCounter) (Utilities|Array|Length _dialogue))
        (if (Variables|Default|GetOpenRNGLevel)
          (bind _outactors (Actor|GetAllActorswithInterface "/Game/Blueprints/UtilityItems/BP_ExitInterface.BP_ExitInterface_C"))
          (Class|BPExitInterface|Exit(Message) (Utilities|Array|Get(acopy) _outactors) "None")
          (else
            (if (Variables|Default|GetChangeToSpecificLevelAfterDialogue) :!label _label_2
              (if (== _nextscenename "")
                (Development|PrintString "Next Scene Name is None, Opening Test Map")
                (Game|OpenLevel(byName) "TestMap")
                (else
                  (Game|OpenLevel(byName) _nextscenename)))
              (else
                (CallFunction|EndDialogue)
                (if (Variables|Default|GetFreezeAIUntilAfterDialogue)
                  (if (Variables|Default|GetDelayUnfreezeAI)
                    (Utilities|FlowControl|Delay 0.2)
                    (CallFunction|DelayUnfreezeAIFunc)
                    (else
                      (Default|UnfreezeAI (Variables|Default|GetBP%20Player%20Movement) false))))
                (if (Variables|Default|GetFreezePlayerUntilAfterDialogue)
                  (Default|UnfreezePlayer (Variables|Default|GetBP%20Player%20Movement)))))
            (if (Variables|Default|GetTutorialMapLevel1)
              (Variables|/Script/ExtractShooter.PlayerMovement|SetisInDialogue (Variables|Default|GetBP%20Tutorial%20Player) false)
              (else
                (Variables|/Script/ExtractShooter.PlayerMovement|SetisInDialogue (Variables|Default|GetBP%20Player%20Movement) false)))))
        (else
          (bind _asbp_game_instance (Utilities|Casting|CastToBP_GameInstance (Game|GetGameInstance)))
          (if (Variables|/Game/Blueprints/BP_GameInstance.BP_GameInstance_C|GetDontPlayDialogue _asbp_game_instance)
            (CallFunction|EndDialogue)
            (goto _label_2)
            (else
              (if (== (Variables|Default|GetBP%20Player%20Movement) 0) :!label _label_3
                (bind _returnvalue_2 (Actor|GetActorOfClass "/Game/Blueprints/Player/BP_PlayerMovement.BP_PlayerMovement_C"))
                (Variables|Default|SetBP%20Player%20Movement _returnvalue_2)
                (Utilities|FlowControl|Delay 0.2)
                (goto _label_3)
                (else
                  (Default|TogglePopupTextVisibility (Variables|/Game/Blueprints/Player/BP_PlayerMovement.BP_PlayerMovement_C|GetPlayerUI (Variables|Default|GetBP%20Player%20Movement)) true)
                  (CallFunction|TypeWriterText _output_get_2 _output_get_3)
                  (Variables|Default|SetTypeWriterCounterLocal (Variables|Default|GetCounter))
                  (Variables|Default|SetCounter (+ (Variables|Default|GetCounter) 1)))))))))))

(event Custom|PlaceImagesInWidget
  (params (NameString :type String) (DialogueString :type String))
  (bind _bp_dialogue_widget (Variables|Default|GetBP%20Dialogue%20Widget))
  (bind _bp_dialogue_widget_2 (Variables|Default|GetBP%20Dialogue%20Widget))
  (bind _nameimage (Variables|/Game/Blueprints/UI/BP_DialogueWidget.BP_DialogueWidget_C|GetNameImage _bp_dialogue_widget))
  (bind _dialogueimage (Variables|/Game/Blueprints/UI/BP_DialogueWidget.BP_DialogueWidget_C|GetDialogueImage _bp_dialogue_widget_2))
  (if (Utilities|Enum|Equal(Enum) NameString "")
    (Class|Image|SetOpacity _nameimage 0.0)
    (else
      (Class|Image|SetOpacity _nameimage 1.0)))
  (if (Utilities|Enum|Equal(Enum) DialogueString "")
    (Class|Image|SetOpacity _dialogueimage 0.0)
    (else
      (Class|Image|SetOpacity _dialogueimage 1.0))))

(event Custom|TypeWriterText
  (params (Name :type String) (Dialogue :type String))
  (bind _bp_dialogue_widget (Variables|Default|GetBP%20Dialogue%20Widget))
  (bind _bp_dialogue_widget_2 (Variables|Default|GetBP%20Dialogue%20Widget))
  (bind _dialoguetext (Variables|/Game/Blueprints/UI/BP_DialogueWidget.BP_DialogueWidget_C|GetDialogueText _bp_dialogue_widget))
  (bind _dialoguetext_2 (Variables|/Game/Blueprints/UI/BP_DialogueWidget.BP_DialogueWidget_C|GetDialogueText _bp_dialogue_widget_2))
  (Rendering|Components|TextRender|SetText (Variables|/Game/Blueprints/UI/BP_PlayerUI.BP_PlayerUI_C|GetPopupTextUI (Variables|/Game/Blueprints/Player/BP_PlayerMovement.BP_PlayerMovement_C|GetPlayerUI (Variables|Default|GetBP%20Player%20Movement))) "")
  (Rendering|Components|TextRender|SetText _dialoguetext_2 "")
  (Rendering|Components|TextRender|SetText (Variables|/Game/Blueprints/UI/BP_DialogueWidget.BP_DialogueWidget_C|GetNameText _bp_dialogue_widget_2) (Utilities|Text|ToText(String) Name))
  (Utilities|FlowControl|Delay (Variables|Default|GetCharacterPerSecond) :!label _label)
  (Utilities|FlowControl|Sequence
    (:then_0
      (if (Variables|/Script/ExtractShooter.PlayerMovement|GetisInDialogue (Variables|Default|GetBP%20Player%20Movement))
        ;[1 1 1] One more character shown
        (Rendering|Components|TextRender|SetText _dialoguetext (Utilities|Text|ToText(String) (Utilities|String|GetSubstring Dialogue 0 (+ (Utilities|String|Len (Utilities|String|ToString(Text) (Class|TextBlock|GetText _dialoguetext))) 1))))
        (elif (not (Variables|Default|GetLockDialogue))
          (CallFunction|EndDialogue))))
    (:then_1
      (if (Utilities|Enum|Equal(Enum) Dialogue (Utilities|String|ToString(Text) (Class|TextBlock|GetText _dialoguetext_2)))
        (Default|PopupTextDuringDialogue (Variables|/Game/Blueprints/Player/BP_PlayerMovement.BP_PlayerMovement_C|GetPlayerUI (Variables|Default|GetBP%20Player%20Movement)) (Utilities|String|ToString(Text) (Utilities|Array|Get(acopy) (Variables|Default|GetPopupTextDuringDialogue) (Variables|Default|GetTypeWriterCounterLocal))))
        (else
          (goto _label))))))

(event Custom|DelayUnfreezeAIFunc
  (bind _returnvalue (Actor|GetActorOfClass "/Game/Blueprints/Player/BP_PlayerMovement.BP_PlayerMovement_C"))
  (Default|FreezeAI _returnvalue)
  (Development|PrintString "FREEZE AI DELAY UINFREEZE AI")
  (Utilities|FlowControl|Delay (Variables|Default|GetDelayUnfreezeAITime))
  (Default|UnfreezeAI _returnvalue true)
  (Development|PrintString "UNFROZE AI FROM DELAY"))

(event EventBeginPlay
  (bind _asbp_game_instance (Utilities|Casting|CastToBP_GameInstance (Game|GetGameInstance)))
  (if (not (Variables|/Game/Blueprints/BP_GameInstance.BP_GameInstance_C|GetHasPlayedDialogue _asbp_game_instance))
    (if (and (and (Variables|Default|GetNoCutscene) (Variables|Default|GetOnBeginPlay)) (== (Variables|Default|GetOneTimeEverDialogue) false))
      (if (Variables|Default|GetTutorialMapLevel1)
        (Development|PrintString "DONT USE THIS BP FOR TUTORIALMAPLEVEL1, USE BP TUTORIAL DIALOGUE")
        (else
          (bind _asbp_player_movement (Utilities|Casting|CastToBP_PlayerMovement (Game|GetPlayerCharacter 0) :!label _label)
            (:then
              (Variables|Default|SetBP%20Player%20Movement _asbp_player_movement)
              (if (Variables|/Game/Blueprints/Player/BP_PlayerMovement.BP_PlayerMovement_C|GetLoading (Variables|Default|GetBP%20Player%20Movement)) :!label _label_2
                (Utilities|FlowControl|DelayUntilNextTick)
                (goto _label_2)
                (else
                  (bind _returnvalue (UserInterface|CreateWidget "/Game/Blueprints/UI/BP_DialogueWidget.BP_DialogueWidget_C" (Game|GetPlayerController 0)))
                  (bind _output_get (Variables|Default|SetBP%20Dialogue%20Widget _returnvalue))
                  (UserInterface|Viewport|AddtoViewport _output_get 0)
                  (Variables|/Script/ExtractShooter.PlayerMovement|SetisInDialogue (Variables|Default|GetBP%20Player%20Movement) true)
                  (Variables|/Game/Blueprints/Player/BP_PlayerMovement.BP_PlayerMovement_C|SetBP%20Dialogue (Variables|Default|GetBP%20Player%20Movement) self)
                  (CallFunction|NextDialogueNoCutscene))))
            (:CastFailed
              (Development|PrintString "BP PLAYER MOVEMENT CAST FAILED")))))
      (elif (and (and (Variables|Default|GetOneTimeEverDialogue) (Variables|Default|GetOnBeginPlay)) (Variables|Default|GetNoCutscene))
        (bind _asbp_game_instance_2 (Utilities|Casting|CastToBP_GameInstance (Game|GetGameInstance)))
        (if (Variables|/Game/Blueprints/BP_GameInstance.BP_GameInstance_C|GetOneTimeEverDialogue _asbp_game_instance_2)
          (Development|PrintString "BP DIALOGUE ONE TIME EVER DIALOGUE TRUE, BP GAME INSTANCE ONE TIME EVER DIALOGUE IS ALREADY TRUE. NOT PLAYING DIALOGUE")
          (else
            (Variables|/Game/Blueprints/BP_GameInstance.BP_GameInstance_C|SetOneTimeEverDialogue _asbp_game_instance_2 true)
            (goto _label)))
        (elif (and (not (Variables|Default|GetNoCutscene)) (Variables|Default|GetOnBeginPlay))
          (bind _returnvalue_2 (Actor|GetActorOfClass "/Game/Blueprints/Cutscene/BP_PlayerMovementCutscene.BP_PlayerMovementCutscene_C" :!label _label_3))
          (bind _returnvalue_3 (UserInterface|CreateWidget "/Game/Blueprints/UI/BP_DialogueWidget.BP_DialogueWidget_C"))
          (bind _output_get_2 (Variables|Default|SetBP%20Dialogue%20Widget _returnvalue_3))
          (UserInterface|Viewport|AddtoViewport _output_get_2 0)
          (bind _returnvalue_4 (Actor|GetActorOfClass "/Game/Blueprints/Cutscene/BP_CutsceneControl.BP_CutsceneControl_C"))
          (Variables|/Game/Blueprints/Cutscene/BP_CutsceneControl.BP_CutsceneControl_C|SetBP%20Dialogue%20Widget _returnvalue_4 _output_get_2)
          (bind _output_get_3 (Variables|Default|SetBP%20Player%20Movement%20Cutscene _returnvalue_2))
          (if (== _output_get_3 0)
            (Development|PrintString "BP PLAYER MOVEMENT CUTSCENE NOT FOUND")
            (Utilities|FlowControl|DelayUntilNextTick)
            (goto _label_3)
            (elif (not (== (Variables|/Game/Blueprints/Cutscene/BP_PlayerMovementCutscene.BP_PlayerMovementCutscene_C|GetBP%20Fade%20Out _output_get_3) 0))
              (if (UserInterface|Viewport|IsinViewport (Variables|/Game/Blueprints/Cutscene/BP_PlayerMovementCutscene.BP_PlayerMovementCutscene_C|GetBP%20Fade%20Out _output_get_3)) :!label _label_4
                (Utilities|FlowControl|DelayUntilNextTick)
                (goto _label_4)
                (else
                  (Variables|/Game/Blueprints/Cutscene/BP_PlayerMovementCutscene.BP_PlayerMovementCutscene_C|SetCanStartDialogue (Variables|Default|GetBP%20Player%20Movement%20Cutscene) true))))))))))

(event Collision|EventActorBeginOverlap
  (params (OtherActor :type Actor%20Object%20Reference)))

(event EventTick
  (params (DeltaSeconds :type Float%20%28single-precision%29)))

(fn ConstructionScript)