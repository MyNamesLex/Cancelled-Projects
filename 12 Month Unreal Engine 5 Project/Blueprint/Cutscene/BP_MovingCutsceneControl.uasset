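; Cutscene controller that pairs a list of Level Sequences with name and dialogue lines from BP_Dialogue.
; On BeginPlay, if that dialogue is set to start automatically, it shows the first line and adds black bars.
; Each NextDialogue plays the next sequence and sets the widget text, retrying on a delay until the widget exists.
; When sequences run out, it clears the text or loads the next level, optionally fading music through BP_AudioManager.
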(event Custom|NextDialogue
  (bind _bp_dialogue (Variables|Default|GetBP%20Dialogue))
  (bind _nextscenename (Variables|/Script/ExtractShooter.Dialogue|GetNextSceneName _bp_dialogue))
  (if (== (Utilities|Array|Get(acopy) (Variables|Default|GetLevelSequence) (Variables|Default|GetCounter)) 0)
    (if (Variables|/Game/Blueprints/Dialogue/BP_Dialogue.BP_Dialogue_C|GetChangeToSpecificLevelAfterDialogue (Variables|Default|GetBP%20Dialogue))
      (if (Variables|Default|GetFadeOutAudio)
        (Default|FadeOutBGMLoadNextLevel (Variables|Default|GetBP%20Audio%20Manager) 1.0 _nextscenename)
        (else
          (Game|OpenLevel(byName) _nextscenename)))
      (else
        (CallFunction|ExitDialogue)))
    (else
      (if (Audio|Components|Audio|IsPlaying (Variables|Default|GetLevelSequencePlayer))
        (Sequencer|Player|Stop (Variables|Default|GetLevelSequencePlayer) :!class /Script/MovieScene.MovieSceneSequencePlayer))
      (bind (_outactor _returnvalue) (Sequencer|Player|CreateLevelSequencePlayer (Utilities|Array|Get(acopy) (Variables|Default|GetLevelSequence) (Variables|Default|GetCounter))))
      (Variables|Default|SetLevelSequencePlayer _returnvalue)
      (Sequencer|Player|Play (Variables|/Script/LevelSequence.LevelSequenceActor|GetSequencePlayer _outactor) :!class /Script/MovieScene.MovieSceneSequencePlayer)
      (bind _output_get (Variables|Default|SetName (Utilities|Array|Get(acopy) (Variables|/Script/ExtractShooter.Dialogue|GetName _bp_dialogue) (Variables|Default|GetCounter))))
      (bind _output_get_2 (Variables|Default|SetDialogue (Utilities|Array|Get(acopy) (Variables|/Script/ExtractShooter.Dialogue|GetDialogue _bp_dialogue) (Variables|Default|GetCounter))))
      (Variables|Default|SetCounter (+ (Variables|Default|GetCounter) 1))
      (if (== (Variables|Default|GetBP%20Dialogue%20Widget) 0) :!label _label
        (Variables|Default|SetBP%20Dialogue%20Widget (Variables|/Game/Blueprints/Dialogue/BP_Dialogue.BP_Dialogue_C|GetBP%20Dialogue%20Widget (Variables|Default|GetBP%20Dialogue)))
        (Utilities|FlowControl|Delay 0.2)
        (goto _label)
        (else
          (Rendering|Components|TextRender|SetText (Variables|/Game/Blueprints/UI/BP_DialogueWidget.BP_DialogueWidget_C|GetNameText (Variables|Default|GetBP%20Dialogue%20Widget)) (Utilities|Text|ToText(String) _output_get))
          (Rendering|Components|TextRender|SetText (Variables|/Game/Blueprints/UI/BP_DialogueWidget.BP_DialogueWidget_C|GetDialogueText (Variables|Default|GetBP%20Dialogue%20Widget)) (Utilities|Text|ToText(String) _output_get_2)))))))

(event Custom|Exit%20Dialogue
  (bind _bp_dialogue_widget (Variables|Default|GetBP%20Dialogue%20Widget))
  (Rendering|Components|TextRender|SetText (Variables|/Game/Blueprints/UI/BP_DialogueWidget.BP_DialogueWidget_C|GetNameText _bp_dialogue_widget) "")
  (Rendering|Components|TextRender|SetText (Variables|/Game/Blueprints/UI/BP_DialogueWidget.BP_DialogueWidget_C|GetDialogueText _bp_dialogue_widget) ""))

(event Collision|EventActorBeginOverlap
  (params (OtherActor :type Actor%20Object%20Reference)))

(event EventTick
  (params (DeltaSeconds :type Float%20%28single-precision%29)))

(event EventBeginPlay
  (bind _returnvalue (Actor|GetActorOfClass "/Game/Blueprints/Audio/BP_AudioManager.BP_AudioManager_C"))
  (Variables|Default|SetBP%20Audio%20Manager _returnvalue)
  (bind _returnvalue_2 (Actor|GetActorOfClass "/Game/Blueprints/Cutscene/BP_PlayerMovementCutscene.BP_PlayerMovementCutscene_C"))
  (Variables|Default|SetPlayer%20Movement%20Cutscene _returnvalue_2)
  (bind _returnvalue_3 (Actor|GetActorOfClass "/Game/Blueprints/Dialogue/BP_Dialogue.BP_Dialogue_C"))
  (bind _output_get (Variables|Default|SetBP%20Dialogue _returnvalue_3))
  (if (Variables|/Game/Blueprints/Dialogue/BP_Dialogue.BP_Dialogue_C|GetOnBeginPlay _output_get)
    (Variables|Default|SetBP%20Dialogue%20Widget (Variables|/Game/Blueprints/Dialogue/BP_Dialogue.BP_Dialogue_C|GetBP%20Dialogue%20Widget (Variables|Default|GetBP%20Dialogue)))
    (CallFunction|NextDialogue)
    (bind _returnvalue_4 (UserInterface|CreateWidget "/Game/Blueprints/UI/BP_UIBlackBars.BP_UIBlackBars_C"))
    (UserInterface|Viewport|AddtoViewport _returnvalue_4 -99)))

(fn ConstructionScript)