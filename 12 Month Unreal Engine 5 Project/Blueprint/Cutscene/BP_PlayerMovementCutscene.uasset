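; Player input Blueprint for cutscenes that advances dialogue on Enter and skips to the next scene on Slash.
; On BeginPlay it finds the audio manager and either the moving or standard cutscene controller, chosen by MovingCutscene.
; Enter works only while the fade widget is off screen, recreating it before calling NextDialogue.
; Slash opens the dialogue's next scene, optionally fading out BGM first for standard cutscenes.
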(event Custom|ResetBPFadeOut
  (Widget|RemovefromParent (Variables|Default|GetBP%20Fade%20Out))
  (Utilities|FlowControl|DelayUntilNextTick)
  (bind _returnvalue (UserInterface|CreateWidget "/Game/Blueprints/Loading/BP_FadeOut.BP_FadeOut_C"))
  (bind _output_get (Variables|Default|SetBP%20Fade%20Out _returnvalue))
  (Appearance|SetColorandOpacity _output_get (Utilities|Struct|MakeLinearColor 0.0 0.0 0.0 1.0) :!class /Script/UMG.UserWidget)
  (Default|FadeOut _output_get)
  (UserInterface|Viewport|AddtoViewport _output_get 0))

(event EventBeginPlay
  (bind _returnvalue (Actor|GetActorOfClass "/Game/Blueprints/Audio/BP_AudioManager.BP_AudioManager_C"))
  (Variables|Default|SetBP%20Audio%20Manager _returnvalue)
  (if (Variables|Default|GetMovingCutscene?)
    (bind _returnvalue_2 (Actor|GetActorOfClass "/Game/Blueprints/Cutscene/BP_MovingCutsceneControl.BP_MovingCutsceneControl_C"))
    (Variables|Default|SetMovingCutsceneControl _returnvalue_2)
    (else
      (bind _returnvalue_3 (Actor|GetActorOfClass "/Game/Blueprints/Cutscene/BP_CutsceneControl.BP_CutsceneControl_C"))
      (Variables|Default|SetCutsceneControl _returnvalue_3)))
  (bind _returnvalue_4 (UserInterface|CreateWidget "/Game/Blueprints/Loading/BP_FadeOut.BP_FadeOut_C"))
  (bind _output_get (Variables|Default|SetBP%20Fade%20Out _returnvalue_4))
  (UserInterface|Viewport|AddtoViewport _output_get 0)
  (Development|PrintString "Cutscene")
  (Input|SetInputModeGameOnly (Game|GetPlayerController 0)))

(event Collision|EventActorBeginOverlap
  (params (OtherActor :type Actor%20Object%20Reference)))

(event EventTick
  (params (DeltaSeconds :type Float%20%28single-precision%29)))

(event Input|KeyboardEvents|Slash
  (params (Key :type Key%20Structure :default "None"))
  (bind _cutscenecontrol (Variables|Default|GetCutsceneControl))
  (bind _bp_dialogue (Variables|/Game/Blueprints/Cutscene/BP_CutsceneControl.BP_CutsceneControl_C|GetBP%20Dialogue _cutscenecontrol))
  (bind _nextscenename (Variables|/Script/ExtractShooter.Dialogue|GetNextSceneName _bp_dialogue))
  (:Pressed
    (if (Variables|Default|GetMovingCutscene?)
      (Game|OpenLevel(byName) (Variables|/Script/ExtractShooter.Dialogue|GetNextSceneName (Variables|/Game/Blueprints/Cutscene/BP_MovingCutsceneControl.BP_MovingCutsceneControl_C|GetBP%20Dialogue (Variables|Default|GetMovingCutsceneControl))))
      (elif (Variables|/Game/Blueprints/Cutscene/BP_CutsceneControl.BP_CutsceneControl_C|GetFadeOutAudio _cutscenecontrol)
        (Default|FadeOutBGMLoadNextLevel (Variables|Default|GetBP%20Audio%20Manager) 1.0 _nextscenename)
        (else
          (Game|OpenLevel(byName) _nextscenename))))))

(event Input|KeyboardEvents|Enter
  (params (Key :type Key%20Structure :default "None"))
  (:Pressed
    (if (UserInterface|Viewport|IsinViewport (Variables|Default|GetBP%20Fade%20Out))
      (Development|PrintString "BP FADE OUT IN VIEW PORT, BP PLAYERMOVEMENT CUTSCENE ENTER KEY")
      (else
        (Variables|Default|SetCanStartDialogue true)
        (if (Variables|Default|GetCanStartDialogue)
          (CallFunction|ResetBPFadeOut)
          (if (Variables|Default|GetMovingCutscene?)
            (Default|NextDialogue (Variables|Default|GetMovingCutsceneControl))
            (else
              (Default|NextDialogue (Variables|Default|GetCutsceneControl))))
          (else
            (Development|PrintString (Utilities|String|ToString(Boolean) (Variables|Default|GetCanStartDialogue)))))))))

(fn ConstructionScript)