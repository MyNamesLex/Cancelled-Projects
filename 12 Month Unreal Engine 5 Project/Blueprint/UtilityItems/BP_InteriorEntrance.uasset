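; BP_InteriorEntrance is a building entrance trigger that prompts the player to press L and then opens the interior level named by LevelToOpen.
; Box overlap toggles the popup and player flag, while Tick polls LeaveLevel on the main or tutorial player.
; Exit records state through BP_InteriorEntranceManager and BP_GameInstance, then saves stats before loading.
; Exit casts only to BP_PlayerMovement, so the tutorial character never completes the transition.
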(event OnComponentBeginOverlap(Box)
  (params (OverlappedComponent :type Primitive%20Component%20Object%20Reference) (OtherActor :type Actor%20Object%20Reference) (OtherComp :type Primitive%20Component%20Object%20Reference) (OtherBodyIndex :type Integer) (bFromSweep :type Boolean) (SweepResult :type Hit%20Result%20Structure%20%28by%20ref%29))
  (bind _asbp_player_movement (Utilities|Casting|CastToBP_PlayerMovement OtherActor)
    (:then
      (Variables|/Script/ExtractShooter.PlayerMovement|SetOverlappingLevelEnterOrExit _asbp_player_movement true)
      (Variables|Default|Setoverlapping true)
      (Class|PlayerMovement|CallPlayerUIPopupText _asbp_player_movement "Enter Building? \"L\"" 1e+69))
    (:CastFailed
      (bind _asbp_player_movement_tutorial (Utilities|Casting|CastToBP_PlayerMovementTutorial OtherActor))
      (Variables|/Script/ExtractShooter.PlayerMovement|SetOverlappingLevelEnterOrExit _asbp_player_movement_tutorial true)
      (Variables|Default|Setoverlapping true)
      (Class|PlayerMovement|CallPlayerUIPopupText _asbp_player_movement_tutorial "Enter Building? \"L\"" 1e+69))))

(event OnComponentEndOverlap(Box)
  (params (OverlappedComponent :type Primitive%20Component%20Object%20Reference) (OtherActor :type Actor%20Object%20Reference) (OtherComp :type Primitive%20Component%20Object%20Reference) (OtherBodyIndex :type Integer))
  (bind _asbp_player_movement (Utilities|Casting|CastToBP_PlayerMovement OtherActor)
    (:then
      (Variables|/Script/ExtractShooter.PlayerMovement|SetOverlappingLevelEnterOrExit _asbp_player_movement false)
      (Variables|Default|Setoverlapping false)
      (Class|PlayerMovement|CallRemovePlayerUIPopupText _asbp_player_movement))
    (:CastFailed
      (bind _asbp_player_movement_tutorial (Utilities|Casting|CastToBP_PlayerMovementTutorial OtherActor))
      (Variables|/Script/ExtractShooter.PlayerMovement|SetOverlappingLevelEnterOrExit _asbp_player_movement_tutorial false)
      (Variables|Default|Setoverlapping false)
      (Class|PlayerMovement|CallRemovePlayerUIPopupText _asbp_player_movement_tutorial))))

(event Custom|Leave
  (bind _returnvalue (Actor|GetActorOfClass "/Game/Blueprints/Player/BP_PlayerMovement.BP_PlayerMovement_C"))
  (Utilities|Casting|CastToBP_PlayerMovement _returnvalue
    (:then
      (CallFunction|Exit (Variables|Default|GetLevelToOpen)))
    (:CastFailed
      (bind _returnvalue_2 (Actor|GetActorOfClass "/Game/Blueprints/Tutorial/BP_PlayerMovementTutorial.BP_PlayerMovementTutorial_C"))
      (Utilities|Casting|CastToBP_PlayerMovementTutorial _returnvalue_2)
      (CallFunction|Exit (Variables|Default|GetLevelToOpen)))))

(event EventBeginPlay
  (bind _returnvalue (Actor|GetActorOfClass "/Game/Blueprints/UtilityItems/BP_InteriorEntranceManager.BP_InteriorEntranceManager_C"))
  (Variables|Default|SetInterior%20Manager _returnvalue))

(event Collision|EventActorBeginOverlap
  (params (OtherActor :type Actor%20Object%20Reference)))

(event EventTick
  (params (DeltaSeconds :type Float%20%28single-precision%29))
  (if (Variables|Default|Getoverlapping)
    (bind _returnvalue (Actor|GetActorOfClass "/Game/Blueprints/Player/BP_PlayerMovement.BP_PlayerMovement_C"))
    (bind _asbp_player_movement (Utilities|Casting|CastToBP_PlayerMovement _returnvalue)
      (:then
        (Variables|Default|SetPlayer _asbp_player_movement)
        (if (Variables|/Script/ExtractShooter.PlayerMovement|GetLeaveLevel _asbp_player_movement)
          (CallFunction|Leave)))
      (:CastFailed
        (bind _returnvalue_2 (Actor|GetActorOfClass "/Game/Blueprints/Tutorial/BP_PlayerMovementTutorial.BP_PlayerMovementTutorial_C"))
        (bind _asbp_player_movement_tutorial (Utilities|Casting|CastToBP_PlayerMovementTutorial _returnvalue_2))
        (if (Variables|/Script/ExtractShooter.PlayerMovement|GetLeaveLevel _asbp_player_movement_tutorial)
          (CallFunction|Leave))))))

(event EventExit
  (params (LevelToOpen :type Name :default "None"))
  (bind _interior_manager (Variables|Default|GetInterior%20Manager))
  (bind _asbp_game_instance (Utilities|Casting|CastToBP_GameInstance (Game|GetGameInstance)))
  (Variables|/Game/Blueprints/BP_GameInstance.BP_GameInstance_C|SetDontPlayDialogue _asbp_game_instance true)
  (Utilities|Casting|CastToBP_PlayerMovement (Game|GetPlayerCharacter 0))
  (Default|SetDeadEnemiesFunc _interior_manager "None")
  (Default|SetRemovePickedUpItems _interior_manager)
  (bind _asbp_game_instance_2 (Utilities|Casting|CastToBP_GameInstance (Game|GetGameInstance)))
  (Variables|/Game/Blueprints/BP_GameInstance.BP_GameInstance_C|SetStartingPos _asbp_game_instance_2 (Transformation|GetActorTransform (Game|GetPlayerCharacter 0)))
  (Utilities|FlowControl|Delay 0.2)
  (Default|SavePlayerStats (Variables|Default|GetPlayer))
  (Game|OpenLevel(byName) LevelToOpen))

(fn ConstructionScript)