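; BP_RustyTank is an explosive tank prop that damages and stuns AI and players caught in its blast sphere.
; Explode enables sphere overlaps, spawns the effect, plays sound via BP_AudioManager, hides the mesh, then destroys the actor after a short delay.
; Sphere overlaps apply damage and stun, then re-invoke Explode on itself through BP_ExplosionInterface.
; DestroyItem instead teleports it below the world, and Tick keeps the sphere hidden.
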(event OnComponentBeginOverlap(Sphere)
  (params (OverlappedComponent :type Primitive%20Component%20Object%20Reference) (OtherActor :type Actor%20Object%20Reference) (OtherComp :type Primitive%20Component%20Object%20Reference) (OtherBodyIndex :type Integer) (bFromSweep :type Boolean) (SweepResult :type Hit%20Result%20Structure%20%28by%20ref%29))
  (bind _damage (Variables|Default|GetDamage))
  (bind _asbp_aiinterface (Utilities|Casting|CastToBP_AIInterface OtherActor)
    (:then
      (Default|DamageDeal _asbp_aiinterface _damage)
      (Default|Stunned _asbp_aiinterface))
    (:CastFailed
      _))
  (bind _asbp_player_movement (Utilities|Casting|CastToBP_PlayerMovement OtherActor)
    (:then
      (Class|PlayerMovement|DealDamagetoPlayer _asbp_player_movement (Math|Conversions|ToFloat(Integer) _damage))
      (Default|StunnedFunc _asbp_player_movement))
    (:CastFailed
      _))
  (if (== OtherComp 0)
    _
    (else
      _))
  (bind _asbp_explosion_interface (Utilities|Casting|CastToBP_ExplosionInterface self))
  (Default|Explode _asbp_explosion_interface))

(event Custom|DestroyItem
  (Utilities|FlowControl|Delay 0.1)
  (Transformation|SetActorLocation "0, 0,-999.000000" false true))

(event EventBeginPlay
  (bind _returnvalue (Actor|GetActorOfClass "/Game/Blueprints/Audio/BP_AudioManager.BP_AudioManager_C"))
  (Variables|Default|SetBP%20Audio%20Manager _returnvalue))

(event Collision|EventActorBeginOverlap
  (params (OtherActor :type Actor%20Object%20Reference)))

(event EventTick
  (params (DeltaSeconds :type Float%20%28single-precision%29))
  (Rendering|SetVisibility (Variables|Default|GetSphere) false false))

(event EventExplode
  (bind _rusty_tank (Variables|Default|GetRusty%20Tank))
  (bind _returnvalue (Transformation|GetWorldLocation _rusty_tank))
  (Variables|/Script/Engine.PrimitiveComponent|SetbGenerateOverlapEvents (Variables|Default|GetSphere) true)
  (Niagara|SpawnSystematLocation "/Game/Assets/Niagara/Traps/Outer_Mine_Explosion.Outer_Mine_Explosion" _returnvalue "0, 0, 0" "2.000000,2.000000,2.000000")
  (Default|PlaySFXbyName (Variables|Default|GetBP%20Audio%20Manager) "Explosion" _returnvalue)
  (Rendering|SetVisibility (Variables|Default|GetRusty%20Tank) false false)
  (Utilities|FlowControl|Delay 0.2)
  (Actor|DestroyActor))

(fn ConstructionScript)