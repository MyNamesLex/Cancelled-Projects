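; BP_ChoiceImpact is an actor that handles choice consequences: positive or negative outcomes, inventory item removal and level transitions.
; It caches the player and inventory widget on BeginPlay and every Tick.
; String chances convert to integers, then a random roll against the fail chance sets the effect flags.
; Level loading opens a named level, or retries BP_LevelTracker for a random one when given "None".
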(event EventBeginPlay
  (bind _asbp_player_movement (Utilities|Casting|CastToBP_PlayerMovement (Game|GetPlayerCharacter 0))
    (:then
      (bind _output_get (Variables|Default|SetPlayer _asbp_player_movement))
      (Variables|Default|SetInventory%20Widget (Variables|/Game/Blueprints/Player/BP_PlayerMovement.BP_PlayerMovement_C|GetInventoryWidget _output_get))
      (Variables|Default|SetPlayerVar _output_get))
    (:CastFailed
      (Development|PrintString "PLAYER CAST FAILED"))))

(event Collision|EventActorBeginOverlap
  (params (OtherActor :type Actor%20Object%20Reference)))

(event EventTick
  (params (DeltaSeconds :type Float%20%28single-precision%29))
  (bind _asbp_player_movement (Utilities|Casting|CastToBP_PlayerMovement (Game|GetPlayerCharacter 0)))
  (bind _output_get (Variables|Default|SetPlayer _asbp_player_movement))
  (Variables|Default|SetInventory%20Widget (Variables|/Game/Blueprints/Player/BP_PlayerMovement.BP_PlayerMovement_C|GetInventoryWidget _output_get)))

(event EventRemoveItemfromInventory
  (params (Index :type Integer))
  (bind _inventory_widget (Variables|Default|GetInventory%20Widget))
  (bind _player (Variables|Default|GetPlayer))
  (bind _itemarray (Variables|/Game/Blueprints/Player/BP_PlayerMovement.BP_PlayerMovement_C|GetItemArray _player))
  (bind _listvertical (Variables|/Game/Blueprints/Inventory/BP_InventoryWidget.BP_InventoryWidget_C|GetListVertical _inventory_widget))
  (Development|PrintString "REMOVE ITEM FROM INVENTORY CALLED")
  (Default|RemoveStoredItemVarsinArrays _inventory_widget Index)
  (Utilities|Array|RemoveItem _itemarray (Utilities|Array|Get(acopy) _itemarray (Variables|/Game/Blueprints/Player/BP_PlayerMovement.BP_PlayerMovement_C|GetCurrentInvSlot _player)))
  (bind _returnvalue (Class|PanelWidget|RemoveChild _listvertical (Utilities|Array|Get(acopy) (Class|PanelWidget|GetAllChildren _listvertical) Index)))
  (if _returnvalue
    (Default|GetCurrentWeaponStats _player)
    (Default|FixInventorySorting _inventory_widget)
    (Development|PrintString "ITEM REMOVED")
    (else
      (Development|PrintString "ITEM NOT REMOVED"))))

(event EventLeveltoLoad
  (params (LevelName :type Name :default "None"))
  (if (== LevelName "")
    (bind _returnvalue (Actor|GetActorOfClass "/Game/Blueprints/UtilityItems/BP_LevelTracker.BP_LevelTracker_C"))
    (bind _levelname (Default|GetRandomLevelName _returnvalue :!label _label))
    (if (or (Utilities|Enum|Equal(Enum) (Utilities|String|ToString(Name) _levelname) "None") (Utilities|Enum|Equal(Enum) (Utilities|String|ToString(Name) _levelname) ""))
      (Utilities|FlowControl|Delay 0.2)
      (goto _label)
      (else
        (Development|PrintString (Utilities|String|ToString(Name) _levelname))
        (Game|OpenLevel(byName) _levelname)))
    (else
      (Game|OpenLevel(byName) LevelName))))

(event EventFStringChancestoInt
  (Variables|Default|SetSuccessChanceInt (Math|Conversions|ToInteger(Byte) (Variables|Default|GetSuccessChance)))
  (Variables|Default|SetFailChanceInt (Math|Conversions|ToInteger(Byte) (Variables|Default|GetFailChance)))
  (Class|ChoiceImpact|SetPositiveorNegative))

(event EventSetPositiveorNegative
  (bind _output_get (Variables|Default|SetFalse (<= (Math|Random|RandomFloatinRange 0.0 1e+02) (Variables|Default|GetFailChanceInt))))
  (if _output_get
    (Variables|Default|SetShowPositiveEffect false)
    (Variables|Default|SetShowNegativeEffect true)
    (Development|PrintString "NEGATIVE EFFECT")
    (else
      (Variables|Default|SetShowPositiveEffect true)
      (Variables|Default|SetShowNegativeEffect false)
      (Development|PrintString "POSITIVE EFFECT")))
  (if (not (== (== (Variables|Default|GetShowPositiveEffect) (Variables|Default|GetShowNegativeEffect)) false))
    (Development|PrintString "SHOW POSITIVE EFFECT AND NEGATIVE EFFECT = FALSE")))

(fn ConstructionScript)